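; Camera mode in the Tempest Combat Framework demo that, going by its name, frames executions on random mobs with an offset, shortened spring arm and camera lag disabled.
; It builds its camera property objects on start and ticks through TempestTickingComponent, switching on a status tag.
; Looping processes every property.
; Ending curve-blends the arm back to defaults while processing control rotation, then restores lag and switches to the melee camera mode.
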(event EventOnUpdatedCameraModeStatus
  (bind _cameramodecomponent (Variables|Default|GetCameraModeComponent))
  (bind _springarmcomponent (Variables|/Script/TempestCameraSystems.TempestCameraModeComponent|GetSpringArmComponent _cameramodecomponent))
  (|SwitchGameplayTag (Variables|Default|GetCameraModeStatus)
    (:Camera.Mode.Status.Looping
      (bind _asbp_socket_offset_camera_property (Utilities|Casting|CastToBP_SocketOffsetCameraProperty (Class|TempestBaseCameraMode|GetCameraPropertyOfType "(TagName=\"Property.Camera.Socket Offset\")")))
      (Variables|/Game/TCF_SampleDemo/TempestCombatFramework/Camera/BP_SocketOffsetCameraProperty.BP_SocketOffsetCameraProperty_C|SetTarget%20Value _asbp_socket_offset_camera_property "0.000000,-60.000000,10.000000")
      (bind _asbp_spring_arm_camera_property (Utilities|Casting|CastToBP_SpringArmCameraProperty (Class|TempestBaseCameraMode|GetCameraPropertyOfType "(TagName=\"Property.Camera.Spring Arm\")")))
      (Variables|/Game/TCF_SampleDemo/TempestCombatFramework/Camera/BP_SpringArmCameraProperty.BP_SpringArmCameraProperty_C|SetTarget%20Value _asbp_spring_arm_camera_property 3e+02))
    (:Camera.Mode.Status.Ending
      (Variables|Default|SetTimePassed 0.0)
      (Variables|Default|SetStart%20Socket%20Offset (Variables|/Script/Engine.SpringArmComponent|GetSocketOffset _springarmcomponent))
      (Variables|Default|SetStartTarget%20Arm%20Length (Variables|/Script/Engine.SpringArmComponent|GetTargetArmLength _springarmcomponent))
      (Variables|Default|SetStart%20Control%20Rotation (Pawn|GetControlRotation (Variables|Default|GetPlayer%20Controller) :!class /Script/Engine.Controller)))))

(event EventTickTempestObject
  (params (Value :type Float%20%28single-precision%29))
  (bind _cameramodecomponent (Variables|Default|GetCameraModeComponent))
  (bind _cameramodecomponent_2 (Variables|Default|GetCameraModeComponent))
  (bind _springarmcomponent (Variables|/Script/TempestCameraSystems.TempestCameraModeComponent|GetSpringArmComponent _cameramodecomponent))
  (if (== (Variables|/Script/TempestCameraSystems.TempestCameraModeComponent|GetCurrentCameraMode _cameramodecomponent_2) self)
    (|SwitchGameplayTag (Variables|Default|GetCameraModeStatus)
      (:Camera.Mode.Status.Looping
        (for _array_element (Variables|Default|GetCameraProperties)
          (Class|TempestBaseCameraProperty|ProcessCameraProperty (Utilities|Struct|BreakInstancedCameraProperty _array_element))))
      (:Camera.Mode.Status.Ending
        (Variables|/Script/Engine.SpringArmComponent|SetSocketOffset _springarmcomponent (Math|Vector|Lerp(Vector) (Variables|Default|GetStart%20Socket%20Offset) "0, 0,60.000000" (Math|Curves|GetFloatValue (Variables|Default|GetReset%20Float%20Curve) (Variables|Default|GetTimePassed))))
        (Variables|/Script/Engine.SpringArmComponent|SetTargetArmLength _springarmcomponent (Math|Float|Lerp (Variables|Default|GetStartTarget%20Arm%20Length) 3.7e+02 (Math|Curves|GetFloatValue (Variables|Default|GetReset%20Float%20Curve) (Variables|Default|GetTimePassed))))
        (Class|TempestBaseCameraProperty|ProcessCameraProperty (Class|TempestBaseCameraMode|GetCameraPropertyOfType "(TagName=\"Property.Camera.Control Rotation\")"))
        (if (>= (Math|Curves|GetFloatValue (Variables|Default|GetReset%20Float%20Curve) (Variables|Default|GetTimePassed)) 1.0)
          (Class|TempestBaseCameraMode|SetCameraModeStatus "(TagName=\"Camera.Mode.Status.Nothing\")")
          (Class|TempestCameraModeComponent|SetCameraModeOfClass (Variables|Default|GetCameraModeComponent) "/TempestCombatFramework/Camera/Modes/BP_MeleeCameraMode.BP_MeleeCameraMode_C")
          (Variables|/Script/Engine.SpringArmComponent|SetbEnableCameraLag (Variables|/Script/TempestCameraSystems.TempestCameraModeComponent|GetSpringArmComponent (Variables|Default|GetCameraModeComponent)) true)
          (else
            (Variables|Default|SetTimePassed (+ (Variables|Default|GetTimePassed) Value))))))
    (else
      (Class|TempestTickingComponent|RemoveTickableObject (Actor|GetComponentbyClass (Components|GetOwner _cameramodecomponent_2) "/Script/TempestCore.TempestTickingComponent") self))))

(event EventStartCameraMode
  (bind _ascharacter (Utilities|Casting|CastToCharacter (Components|GetOwner (Variables|Default|GetCameraModeComponent))))
  (bind _asplayer_controller (Utilities|Casting|CastToPlayerController (Pawn|GetController _ascharacter)))
  (Variables|Default|SetPlayer%20Controller _asplayer_controller)
  (Variables|/Script/Engine.SpringArmComponent|SetbEnableCameraLag (Variables|/Script/TempestCameraSystems.TempestCameraModeComponent|GetSpringArmComponent (Variables|Default|GetCameraModeComponent)) false)
  (for _array_element (Variables|Default|GetCameraProperties)
    (Class|TempestBaseCameraProperty|SetCameraMode (Utilities|Struct|BreakInstancedCameraProperty _array_element) (Variables|/Script/TempestCameraSystems.TempestCameraModeComponent|GetCurrentCameraMode (Variables|Default|GetCameraModeComponent)))
    (Class|TempestBaseCameraProperty|ConstructCameraProperty (Utilities|Struct|BreakInstancedCameraProperty _array_element))
    (Class|TempestBaseCameraProperty|StartCameraProperty (Utilities|Struct|BreakInstancedCameraProperty _array_element)))
  (Class|TempestBaseCameraMode|SetCameraModeStatus "(TagName=\"Camera.Mode.Status.Looping\")")
  (Class|TempestTickingComponent|AddTickableObject (Actor|GetComponentbyClass (Components|GetOwner (Variables|Default|GetCameraModeComponent)) "/Script/TempestCore.TempestTickingComponent") self))