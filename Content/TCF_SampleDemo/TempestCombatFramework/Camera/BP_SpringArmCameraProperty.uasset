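; Camera property in the Tempest Combat Framework that smoothly adjusts the spring arm length of its camera mode.
; Starting the property sets its status to Stage One.
; Processing interpolates the camera mode component's TargetArmLength toward a target value with FInterpTo, using frame delta time and a configurable speed.
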(event EventStartCameraProperty
  (Class|TempestBaseCameraProperty|UpdateCameraPropertyStatus "(TagName=\"Camera.Property.Status.Stage.One\")"))

(event EventProcessCameraProperty
  (bind _cameramode (Variables|Default|GetCameraMode))
  (bind _cameramodecomponent (Variables|/Script/TempestCameraSystems.TempestBaseCameraMode|GetCameraModeComponent _cameramode))
  (bind _springarmcomponent (Variables|/Script/TempestCameraSystems.TempestCameraModeComponent|GetSpringArmComponent _cameramodecomponent))
  (|SwitchGameplayTag (Variables|Default|GetCameraPropertyStatus)
    (:Default
      _)
    (:Camera.Property.Status.Stage.One
      _))
  (Variables|/Script/Engine.SpringArmComponent|SetTargetArmLength _springarmcomponent (Math|Interpolation|FInterpTo (Variables|/Script/Engine.SpringArmComponent|GetTargetArmLength _springarmcomponent) (Variables|Default|GetTarget%20Value) (Utilities|Time|GetWorldDeltaSeconds) (Variables|Default|GetInterp%20Speed))))