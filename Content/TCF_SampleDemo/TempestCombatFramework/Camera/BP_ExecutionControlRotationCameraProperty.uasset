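; Camera property for the Tempest Combat Framework that smoothly turns the player's control rotation during executions.
; On start it caches the character's forward and right vectors and enters stage one.
; While processing, it interpolates control rotation toward their normalized sum, a fixed heading 45 degrees right of the initial facing.
; Construction stores the first nearby character from a sphere overlap, but the rotation math does not use it.
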(event EventProcessCameraProperty
  (bind _returnvalue (Game|GetPlayerController 0))
  (bind _returnvalue_2 (Pawn|GetControlRotation _returnvalue :!class /Script/Engine.Controller))
  (|SwitchGameplayTag (Variables|Default|GetCameraPropertyStatus)
    (:Default
      _)
    (:Camera.Property.Status.Stage.One
      _))
  (Pawn|SetControlRotation _returnvalue (Math|Interpolation|RInterpTo _returnvalue_2 (Math|Rotator|Lerp(Rotator) _returnvalue_2 (Math|Conversions|RotationFromXVector (Math|Vector|Normalize (+ (* (stale EventStartCameraProperty _output_get) 1.0) (stale EventStartCameraProperty _output_get_2)))) 1.0 true) (Utilities|Time|GetWorldDeltaSeconds) (Variables|Default|GetInterp%20Speed))))

(event EventConstructCameraProperty
  (bind _cameramode (Variables|Default|GetCameraMode))
  (bind _cameramodecomponent (Variables|/Script/TempestCameraSystems.TempestBaseCameraMode|GetCameraModeComponent _cameramode))
  (bind _returnvalue (Components|GetOwner _cameramodecomponent))
  (bind _outactors (Collision|SphereOverlapActors (Transformation|GetActorLocation _returnvalue) 2.5e+02 (Utilities|Array|MakeArray "ObjectTypeQuery3") "/Script/Engine.Character" (Utilities|Array|MakeArray _returnvalue)))
  (Variables|Default|SetHit%20Actor (Utilities|Array|Get(acopy) _outactors)))

(event EventStartCameraProperty
  (bind _returnvalue (Game|GetPlayerCharacter 0))
  (bind _output_get (Variables|Default|SetRight%20Vector (Transformation|GetActorRightVector _returnvalue)))
  (bind _output_get_2 (Variables|Default|SetForward%20Vector (Transformation|GetActorForwardVector _returnvalue)))
  (Variables|Default|SetSpring%20Arm%20Rotation (Transformation|GetWorldRotation (Variables|/Script/TempestCameraSystems.TempestCameraModeComponent|GetSpringArmComponent (Variables|/Script/TempestCameraSystems.TempestBaseCameraMode|GetCameraModeComponent (Variables|Default|GetCameraMode)))))
  (Class|TempestBaseCameraProperty|UpdateCameraPropertyStatus "(TagName=\"Camera.Property.Status.Stage.One\")"))