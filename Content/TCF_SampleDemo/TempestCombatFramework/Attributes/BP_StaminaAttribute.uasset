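; Stamina attribute for the Tempest Combat Framework that keeps its attribute modifier in step with the current stamina value.
; It extends ModifyAttribute, running the parent logic, then looking up the Attribute.Modifier.Stamina modifier on the owner's attributes component.
; If that modifier is valid, it restarts while stamina is below maximum and stops once stamina reaches maximum.
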(event EventModifyAttribute
  (params (ModifyBy :type Float%20%28single-precision%29))
  (bind _currentowningactor (Class|TempestBaseAttributeObject|GetOwningActor))
  (bind _attributevalues (Variables|Default|GetAttributeValues))
  (bind _returnvalue (Actor|GetComponentbyClass _currentowningactor "/TempestCombatFramework/Components/BP_TempestAttributesComponents.BP_TempestAttributesComponents_C"))
  (bind _foundattributemodifier (Class|TempestAttributesComponents|GetAttributeModifierOfGamplayTag _returnvalue "(TagName=\"Attribute.Modifier.Stamina\")"))
  (|CallParentFunction ModifyBy)
  (Utilities|IsValid _foundattributemodifier
    (:Is%20Valid
      (if (< (.attributevalue _attributevalues) (.maxattributevalue _attributevalues))
        (Class|TempestBaseAttributeModifier|RestartAttributeModifier _foundattributemodifier)
        (elif (>= (.attributevalue _attributevalues) (.maxattributevalue _attributevalues))
          (Class|TempestBaseAttributeModifier|StopAttributeModifier _foundattributemodifier))))))