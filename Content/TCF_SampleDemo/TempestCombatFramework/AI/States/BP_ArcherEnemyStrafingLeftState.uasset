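; Archer enemy AI state in the Tempest Combat Framework that strafes left, using the negated right vector of its owner.
; When deciding what comes next, it ends itself and randomly picks among restarting, following the target, strafing right or attacking, with attack weighted double.
; Failed picks fall back along a chain: restart to follow, attack to strafe right, and strafe right to restart.
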(fn GetStrafingDirection
  (return (* (Transformation|GetActorRightVector (Variables|Default|GetOwner%20Character)) -1.0)))

(fn DecideNextState
  (bind _tempest_state_manager_component (CallFunction|GetTempestStateManagerComponent))
  (bind _tempest_state_manager_component_2 (CallFunction|GetTempestStateManagerComponent))
  (bind _tempest_state_manager_component_3 (CallFunction|GetTempestStateManagerComponent))
  (Class|TempestBaseStateObject|EndState)
  (switch int (Math|Random|RandomIntegerinRange 0 4)
    (:Default
      (bind _returnvalue (Class|TempestBaseStateManagerComponent|TryPerformStateOfClass _tempest_state_manager_component_3 (Utilities|GetClass (Class|TempestBaseStateManagerComponent|GetStateOfGameplayTag _tempest_state_manager_component_3 "(TagName=\"State.Attack\")")) true))
      (if (not _returnvalue)
        (bind _returnvalue_2 (Class|TempestBaseStateManagerComponent|TryPerformStateOfClass _tempest_state_manager_component_2 (Utilities|GetClass (Class|TempestBaseStateManagerComponent|GetStateOfGameplayTag _tempest_state_manager_component_2 "(TagName=\"State.StrafingRight\")")) true :!label _label))
        (if (not _returnvalue_2)
          (Class|TempestBaseStateObject|RestartState false))))
    (:0
      (bind _returnvalue_3 (Class|TempestBaseStateObject|RestartState true))
      (if (not _returnvalue_3)
        (Class|TempestBaseStateManagerComponent|TryPerformStateOfClass _tempest_state_manager_component (Utilities|GetClass (Class|TempestBaseStateManagerComponent|GetStateOfGameplayTag _tempest_state_manager_component "(TagName=\"State.FollowTarget\")")) true :!label _label_2)))
    (:1
      (goto _label_2))
    (:2
      (goto _label))))