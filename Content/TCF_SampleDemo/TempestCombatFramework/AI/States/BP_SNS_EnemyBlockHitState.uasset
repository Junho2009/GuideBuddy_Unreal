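; Enemy AI state for reacting to a blocked hit in the Tempest Combat Framework.
; It can run only if an ability associated with the List.One tag can run, and on start it performs the selected ability.
; Starting also adds one to the owner's block-hit count statistic, if that statistic exists.
; When deciding the next state, it attempts a condition-checked switch to the FollowTarget state.
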(event EventStartState
  (bind _owner_character (Variables|Default|GetOwner%20Character))
  (bind _returnvalue (Actor|GetComponentbyClass _owner_character "/Script/TempestCombatFramework.TempestStatisticsComponent"))
  (bind _foundstatistic (Class|TempestStatisticsComponent|GetStatisticOfGameplayTag _returnvalue "(TagName=\"Statistic.Count.Block Hit\")"))
  (|CallParentFunction)
  (Class|TempestBaseAbilityManagerComponent|PerformAbilityOfClass (Actor|GetComponentbyClass (Variables|Default|GetOwner%20Character) "/Script/TempestCombatFramework.TempestBaseAbilityManagerComponent") (CallFunction|GetSelectedAbility))
  (Utilities|IsValid _returnvalue
    (:Is%20Valid
      (Utilities|IsValid _foundstatistic
        (:Is%20Valid
          (Class|TempestBaseStatisticObject|UpdateStatisticValueby _foundstatistic 1.0))))))

(fn DecideNextState
  (bind _tempest_state_manager_component (CallFunction|GetTempestStateManagerComponent))
  (Class|TempestBaseStateManagerComponent|TryPerformStateOfClass _tempest_state_manager_component (Utilities|GetClass (Class|TempestBaseStateManagerComponent|GetStateOfGameplayTag _tempest_state_manager_component "(TagName=\"State.FollowTarget\")")) true))

(fn CanPerformState
  (bind _return_value (CallFunction|CheckCanRunAssociatedAbilitiesOfTag "(TagName=\"List.One\")"))
  (return _return_value))