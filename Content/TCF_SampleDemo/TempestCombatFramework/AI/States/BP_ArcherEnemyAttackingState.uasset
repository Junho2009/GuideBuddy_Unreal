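; Attacking state for the archer enemy AI in the Tempest Combat Framework, which performs a selected ability through the actor's ability manager on start.
; It can run only with a valid combat target and a passing associated-ability check, plus a coin flip when already active.
; When deciding the next state it tries turning, then restarting itself, then a random left or right strafe, and finally following the target.
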(event EventStartState
  (|CallParentFunction)
  (Class|TempestBaseAbilityManagerComponent|PerformAbilityOfClass (Actor|GetComponentbyClass (Class|TempestBaseStateObject|GetPerformingActor) "/Script/TempestCombatFramework.TempestBaseAbilityManagerComponent") (CallFunction|GetSelectedAbility)))

(fn DecideNextState
  (bind _tempest_state_manager_component (CallFunction|GetTempestStateManagerComponent))
  (bind _tempest_state_manager_component_2 (CallFunction|GetTempestStateManagerComponent))
  (|CallParentFunction)
  (bind _returnvalue (Class|TempestBaseStateManagerComponent|TryPerformStateOfClass _tempest_state_manager_component (Utilities|GetClass (Class|TempestBaseStateManagerComponent|GetStateOfGameplayTag _tempest_state_manager_component "(TagName=\"State.Turning\")")) true))
  (if (not _returnvalue)
    (bind _returnvalue_2 (Class|TempestBaseStateObject|RestartState true))
    (if (not _returnvalue_2)
      (bind _returnvalue_3 (Class|TempestBaseStateManagerComponent|TryPerformStateOfClass _tempest_state_manager_component_2 (Utilities|GetClass (Class|TempestBaseStateManagerComponent|GetStateOfGameplayTag _tempest_state_manager_component_2 (select (Math|Random|RandomBool) "(TagName=\"State.StrafingLeft\")" "(TagName=\"State.StrafingRight\")"))) true))
      (if (not _returnvalue_3)
        (Class|TempestBaseStateManagerComponent|TryPerformStateOfClass _tempest_state_manager_component_2 (Utilities|GetClass (Class|TempestBaseStateManagerComponent|GetStateOfGameplayTag _tempest_state_manager_component_2 "(TagName=\"State.FollowTarget\")")) true)))))

(fn CanPerformState
  (Utilities|IsValid (Class|TempestCombatComponent|GetCombatTarget (Actor|GetComponentbyClass (Class|TempestBaseStateObject|GetPerformingActor) "/TempestCombatFramework/Components/BP_TempestBaseCombatComponent.BP_TempestBaseCombatComponent_C"))
    (:Is%20Valid
      (if (CallFunction|GetIsStateCurrentelyActive)
        (bind _return_value (CallFunction|CheckAssociatedAbilitiesOfTag "(TagName=\"List.One\")"))
        (return (and _return_value (Math|Random|RandomBool)))
        (else
          (bind _return_value_2 (CallFunction|CheckAssociatedAbilitiesOfTag "(TagName=\"List.One\")"))
          (return _return_value_2))))
    (:Is%20Not%20Valid
      (return false))))