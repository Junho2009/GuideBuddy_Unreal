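; Archer enemy AI state that strafes right around the combat target for a short random time.
; On activation it takes walk speed from the strafing behavior special property and switches the anim moveset.
; Each tick it moves along the actor's right vector, feeds strafe values to the AnimBP and smoothly turns toward the target.
; DecideNextState randomly picks among restarting, following, attacking or strafing left, with fallbacks.
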(event EventStartState
  (|CallParentFunction)
  (Class|TempestBaseStateObject|StartStateTimer)
  (Variables|Default|SetStateTimeLimit (Math|Random|RandomFloatinRange 1.0 1.5))
  (Class|TempestTickingComponent|AddTickableObject (Actor|GetComponentbyClass (Class|TempestBaseStateObject|GetPerformingActor) "/Script/TempestCore.TempestTickingComponent") self))

(event EventTickTempestObject
  (params (Value :type Float%20%28single-precision%29))
  (bind _returnvalue (CallFunction|GetStrafingDirection))
  (bind _owner_character (Variables|Default|GetOwner%20Character))
  (bind _owner_character_2 (Variables|Default|GetOwner%20Character))
  (bind _returnvalue_2 (Transformation|GetActorRotation _owner_character_2))
  (Utilities|IsValid (Class|TempestCombatComponent|GetCombatTarget (Variables|Default|GetCombat%20Component))
    (:Is%20Valid
      (Pawn|Input|AddMovementInput _owner_character _returnvalue 1.0 false)
      (Class|BPITempestAbilitiesandStates|SetStrafingValues(Message) (Components|SkeletalMesh|GetAnimInstance (Variables|/Script/Engine.Character|GetMesh _owner_character)) (* (.yaw (Math|Rotator|Delta(Rotator) (Transformation|GetActorRotation _owner_character) (Math|Conversions|RotationFromXVector _returnvalue))) -1.0) _returnvalue)
      (Variables|Default|SetActor%20Target (Class|TempestCombatComponent|GetCombatTarget (Variables|Default|GetCombat%20Component)))
      ;[1 1 1] Smooth Rotation
      (Transformation|SetActorRotation _owner_character_2 (Math|Interpolation|RInterpTo (Transformation|GetActorRotation _owner_character_2) (Math|Rotator|MakeRotator (.roll _returnvalue_2) (.pitch _returnvalue_2) (.yaw (Math|Rotator|FindLookatRotation (Transformation|GetActorLocation _owner_character_2) (Transformation|GetActorLocation (Variables|Default|GetActor%20Target))))) (Utilities|Time|GetWorldDeltaSeconds) 28.0)))))

(event EventPreStateActivation
  (bind _owner_character (Variables|Default|GetOwner%20Character))
  (CallFunction|UpdateStrafingMovementSpeed)
  (Variables|/Script/Engine.CharacterMovementComponent|SetMaxWalkSpeed (Variables|/Script/Engine.Character|GetCharacterMovement _owner_character) (Variables|Initialization|GetStrafing%20Movement%20Speed))
  (Class|BPITCFGeneralInterface|AssignMoveset(Message) (Components|SkeletalMesh|GetAnimInstance (Variables|/Script/Engine.Character|GetMesh _owner_character)) "NewEnumerator2"))

(event EventConstructState
  (|CallParentFunction)
  (Variables|Default|SetCombat%20Component (Actor|GetComponentbyClass (Class|TempestBaseStateObject|GetPerformingActor) "/TempestCombatFramework/Components/BP_TempestBaseCombatComponent.BP_TempestBaseCombatComponent_C")))

(fn GetStrafingDirection
  (return (Transformation|GetActorRightVector (Variables|Default|GetOwner%20Character))))

(fn DecideNextState
  (bind _tempest_state_manager_component (CallFunction|GetTempestStateManagerComponent))
  (bind _tempest_state_manager_component_2 (CallFunction|GetTempestStateManagerComponent))
  (bind _tempest_state_manager_component_3 (CallFunction|GetTempestStateManagerComponent))
  (Class|TempestBaseStateObject|EndState)
  (switch int (Math|Random|RandomIntegerinRange 0 4)
    (:Default
      (bind _returnvalue (Class|TempestBaseStateManagerComponent|TryPerformStateOfClass _tempest_state_manager_component_3 (Utilities|GetClass (Class|TempestBaseStateManagerComponent|GetStateOfGameplayTag _tempest_state_manager_component_3 "(TagName=\"State.Attack\")")) true))
      (if (not _returnvalue)
        (bind _returnvalue_2 (Class|TempestBaseStateManagerComponent|TryPerformStateOfClass _tempest_state_manager_component (Utilities|GetClass (Class|TempestBaseStateManagerComponent|GetStateOfGameplayTag _tempest_state_manager_component "(TagName=\"State.StrafingLeft\")")) true :!label _label))
        (if (not _returnvalue_2)
          (Class|TempestBaseStateObject|RestartState false))))
    (:0
      (bind _returnvalue_3 (Class|TempestBaseStateObject|RestartState true))
      (if (not _returnvalue_3)
        (Class|TempestBaseStateManagerComponent|TryPerformStateOfClass _tempest_state_manager_component_2 (Utilities|GetClass (Class|TempestBaseStateManagerComponent|GetStateOfGameplayTag _tempest_state_manager_component_2 "(TagName=\"State.FollowTarget\")")) true :!label _label_2)))
    (:1
      (goto _label_2))
    (:2
      (goto _label))))

(fn UpdateStrafingMovementSpeed
  (bind _owner_character (Variables|Default|GetOwner%20Character))
  (bind _returnvalue (Actor|GetComponentbyClass _owner_character "/Script/TempestCore.TempestPropertiesComponent"))
  (Utilities|IsValid _returnvalue
    (:Is%20Valid
      (for _array_element (Class|TempestPropertiesComponent|GetSpecialProperties _returnvalue)
        (if (== (Variables|/Script/TempestCore.TempestSpecialProperty|GetPropertyTag (Utilities|Struct|BreakInstancedSpecialProperties _array_element)) "(TagName=\"Property.Special.Behavior.Strafing Behavior\")")
          (bind _asbp_enemy_strafing_behavior_property (Utilities|Casting|CastToBP_EnemyStrafingBehaviorProperty (Utilities|Struct|BreakInstancedSpecialProperties _array_element)))
          (Variables|Initialization|SetStrafing%20Movement%20Speed (Variables|/TempestCombatFramework/BehaviorProperties/BP_EnemyStrafingBehaviorProperty.BP_EnemyStrafingBehaviorProperty_C|GetStrafing%20Movement%20Speed _asbp_enemy_strafing_behavior_property))
          (return)))
      (return))))