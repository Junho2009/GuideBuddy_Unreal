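; AI deflect state for the Tempest Combat Framework that runs the character's selected ability through its ability manager on start.
; It can only be performed when an associated ability tagged List.One is able to run.
; When deciding the next state, it tries FollowTarget with a condition check for non-player pawns, while player-controlled pawns go straight to Idle.
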(event EventStartState
  (|CallParentFunction)
  (Class|TempestBaseAbilityManagerComponent|PerformAbilityOfClass (Actor|GetComponentbyClass (Class|TempestBaseStateObject|GetPerformingActor) "/Script/TempestCombatFramework.TempestBaseAbilityManagerComponent") (CallFunction|GetSelectedAbility)))

(fn DecideNextState
  (bind _tempest_state_manager_component (CallFunction|GetTempestStateManagerComponent))
  (bind _tempest_state_manager_component_2 (CallFunction|GetTempestStateManagerComponent))
  (bind _returnvalue (Class|TempestGeneralLibrary|GetIsPawnControlledbyPlayer (Variables|Default|GetOwner%20Character)))
  (if (not _returnvalue)
    (Class|TempestBaseStateManagerComponent|TryPerformStateOfClass _tempest_state_manager_component_2 (Utilities|GetClass (Class|TempestBaseStateManagerComponent|GetStateOfGameplayTag _tempest_state_manager_component_2 "(TagName=\"State.FollowTarget\")")) true)
    (else
      (Class|TempestBaseStateManagerComponent|PerformStateOfClass _tempest_state_manager_component (Utilities|GetClass (Class|TempestBaseStateManagerComponent|GetStateOfGameplayTag _tempest_state_manager_component "(TagName=\"State.Idle\")"))))))

(fn CanPerformState
  (bind _return_value (CallFunction|CheckCanRunAssociatedAbilitiesOfTag "(TagName=\"List.One\")"))
  (return _return_value))