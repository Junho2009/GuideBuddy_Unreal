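; Demo syncing object for Tempest Combat Framework assassinations that moves a target into place in front of the owning character.
; On start it stores the target's transform and computes a point at a set distance along the owner's forward vector, keeping the target's height.
; Each tick it uses the owner float curve to blend location and yaw, turning the target's back to the owner, until the curve's time range ends.
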(event EventConstructSyncingObject
  (|CallParentFunction)
  (bind _ascharacter (Utilities|Casting|CastToCharacter (Variables|Default|GetOwner%20Actor)))
  (Variables|Default|SetOwnerCharacter _ascharacter)
  (CallFunction|StartSyncingObject))

(event EventStartSyncingObject
  (bind _target (Variables|Default|GetTarget))
  (bind _ownercharacter (Variables|Default|GetOwnerCharacter))
  (bind _distance_to_actor (Variables|Default|GetDistance%20To%20Actor))
  (bind _returnvalue (Transformation|GetActorLocation _ownercharacter))
  (bind _returnvalue_2 (Transformation|GetActorForwardVector _ownercharacter))
  (bind _returnvalue_3 (* _returnvalue_2 _distance_to_actor))
  (bind _returnvalue_4 (+ _returnvalue_3 _returnvalue))
  (bind (_x _y) (Math|Vector|BreakVector _returnvalue_4))
  (Variables|Default|SetTime%20Passed 0.0)
  (Variables|Default|SetOriginal%20Value (Transformation|GetActorLocation _target))
  (Variables|Default|SetOriginal%20Rotation (Transformation|GetActorRotation _target))
  (Variables|Default|SetTarget%20Location (Math|Vector|MakeVector _x _y (.Z (Math|Vector|BreakVector (Variables|Default|GetOriginal%20Value)))))
  (Variables|Default|SetStart true))

(event EventTickSyncingObject
  (bind _target (Variables|Default|GetTarget))
  (bind _target_2 (Variables|Default|GetTarget))
  (bind _returnvalue (Transformation|GetActorRotation _target))
  (bind (_roll _pitch) (Math|Rotator|BreakRotator _returnvalue))
  (if (Variables|Default|GetStart)
    (if (not (>= (Variables|Default|GetTime%20Passed) (.MaxTime (Math|Curves|GetTimeRange (Variables|Default|GetOwner%20Float%20Curve)))))
      (Transformation|SetActorRotation _target_2 (Math|Rotator|Lerp(Rotator) (Variables|Default|GetOriginal%20Rotation) (Math|Rotator|MakeRotator _roll _pitch (.yaw (Math|Rotator|FindLookatRotation (Transformation|GetActorLocation (Variables|Default|GetOwnerCharacter)) (Variables|Default|GetTarget%20Location)))) (Math|Curves|GetFloatValue (Variables|Default|GetOwner%20Float%20Curve) (Variables|Default|GetTime%20Passed)) true))
      (Transformation|SetActorLocation _target_2 (Math|Vector|Lerp(Vector) (Variables|Default|GetOriginal%20Value) (Variables|Default|GetTarget%20Location) (Math|Curves|GetFloatValue (Variables|Default|GetOwner%20Float%20Curve) (Variables|Default|GetTime%20Passed))) false false)
      (Variables|Default|SetTime%20Passed (+ (Utilities|Time|GetWorldDeltaSeconds) (Variables|Default|GetTime%20Passed))))))