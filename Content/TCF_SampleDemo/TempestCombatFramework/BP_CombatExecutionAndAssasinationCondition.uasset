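; Combat condition for executions and assassinations that checks whether the owner wields a sword and shield.
; GetConditionResult requires a valid owner and target, then reads the equipped weapon from the owner's BP_TempestBaseCombatComponent.
; It passes only when that weapon's tag equals Weapon.Type.SwordShield; the target is only checked for validity.
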(fn GetConditionResult
  (if (and (Utilities|IsValid (Variables|Default|GetOwner%20Actor)) (Utilities|IsValid (Variables|Default|GetTarget%20Actor)))
    (return (== (Variables|/TempestCombatFramework/Actors/Weapons/BP_BaseWeapon.BP_BaseWeapon_C|GetWeapon%20Tag (Default|GetEquippedWeapon (Actor|GetComponentbyClass (Variables|Default|GetOwner%20Actor) "/TempestCombatFramework/Components/BP_TempestBaseCombatComponent.BP_TempestBaseCombatComponent_C"))) "(TagName=\"Weapon.Type.Sword & Shield\")"))
    (else
      (return false))))