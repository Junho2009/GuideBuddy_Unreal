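; Tempest state for a character being executed.
; It sets an anim instance moveset message before activation, then on start runs the selected ability through the ability manager and makes the capsule ignore the Pawn channel.
; Entry depends on whether abilities associated with a gameplay tag can run.
; Deciding the next state attempts the FollowTarget state with a condition check.
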(event EventStartState
  (|CallParentFunction)
  (Class|TempestBaseAbilityManagerComponent|PerformAbilityOfClass (Actor|GetComponentbyClass (Class|TempestBaseStateObject|GetPerformingActor) "/Script/TempestCombatFramework.TempestBaseAbilityManagerComponent") (CallFunction|GetSelectedAbility))
  (Collision|SetCollisionResponsetoChannel (Variables|/Script/Engine.Character|GetCapsuleComponent (Variables|Default|GetOwner%20Character)) "ECC_Pawn" "ECR_Ignore"))

(event EventPreStateActivation
  (Class|BPITCFGeneralInterface|AssignMoveset(Message) (Components|SkeletalMesh|GetAnimInstance (Variables|/Script/Engine.Character|GetMesh (Variables|Default|GetOwner%20Character))) "NewEnumerator1"))

(fn DecideNextState
  (bind _tempest_state_manager_component (CallFunction|GetTempestStateManagerComponent))
  (Class|TempestBaseStateManagerComponent|TryPerformStateOfClass _tempest_state_manager_component (Utilities|GetClass (Class|TempestBaseStateManagerComponent|GetStateOfGameplayTag _tempest_state_manager_component "(TagName=\"State.FollowTarget\")")) true))

(fn CanPerformState
  (bind _return_value (CallFunction|CheckCanRunAssociatedAbilitiesOfTag "(TagName=\"List.One\")"))
  (return _return_value))