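; Player walking state for the Tempest state manager, valid while the character has velocity and is not falling.
; On start it sets max walk speed from the speeds special property, choosing the in-combat value by combat status tag, and registers for ticking.
; Each tick it lerps yaw toward any targeted component, then tries switching to Falling, otherwise Idle.
; A Sprint transition exists but is unconnected.
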(event EventConstructState
  (|CallParentFunction))

(event EventTickTempestObject
  (params (Value :type Float%20%28single-precision%29))
  (bind _tempest_state_manager_component (CallFunction|GetTempestStateManagerComponent))
  (bind _tempest_state_manager_component_2 (CallFunction|GetTempestStateManagerComponent))
  (CallFunction|RotatetoTargetedActor 0.1)
  (bind _returnvalue (Class|TempestBaseStateManagerComponent|TryPerformStateOfClass _tempest_state_manager_component_2 (Utilities|GetClass (Class|TempestBaseStateManagerComponent|GetStateOfGameplayTag _tempest_state_manager_component_2 "(TagName=\"State.Falling\")")) true))
  (if (not _returnvalue)
    (bind _returnvalue_2 (Class|TempestBaseStateManagerComponent|TryPerformStateOfClass _tempest_state_manager_component (Utilities|GetClass (Class|TempestBaseStateManagerComponent|GetStateOfGameplayTag _tempest_state_manager_component "(TagName=\"State.Idle\")")) true))
    (if (not _returnvalue_2)
      _)))

(event EventStartState
  (|CallParentFunction)
  (CallFunction|UpdateSpeeds)
  (Variables|/Script/Engine.CharacterMovementComponent|SetMaxWalkSpeed (Variables|/Script/Engine.Character|GetCharacterMovement (Variables|Default|GetOwner%20Character)) (Variables|Default|GetWalking%20Movement%20Speed))
  (Class|TempestTickingComponent|AddTickableObject (Actor|GetComponentbyClass (Class|TempestBaseStateObject|GetPerformingActor) "/Script/TempestCore.TempestTickingComponent") self))

(fn CanPerformState
  (return (and (> (Math|Vector|VectorLength (Transformation|GetVelocity (Variables|Default|GetOwner%20Character))) 0.0) (not (AI|Components|NavMovement|IsFalling (Variables|/Script/Engine.Character|GetCharacterMovement (Variables|Default|GetOwner%20Character)))))))

(fn UpdateSpeeds
  (bind _owner_character (Variables|Default|GetOwner%20Character))
  (bind _returnvalue (Actor|GetComponentbyClass _owner_character "/TempestCombatFramework/Components/BP_TempestPropertiesComponent.BP_TempestPropertiesComponent_C"))
  (Utilities|IsValid _returnvalue
    (:Is%20Valid
      (for _array_element (Class|TempestPropertiesComponent|GetSpecialProperties _returnvalue)
        (if (== (Variables|/Script/TempestCore.TempestSpecialProperty|GetPropertyTag (Utilities|Struct|BreakInstancedSpecialProperties _array_element)) "(TagName=\"Property.Special.Speeds\")")
          (bind _asbp_gs_player_speeds_preoperty (Utilities|Casting|CastToBP_GS_PlayerSpeedsPreoperty (Utilities|Struct|BreakInstancedSpecialProperties _array_element)))
          (if (GameplayTags|HasTag (Class|TempestCombatComponent|GetCombatStatus (Actor|GetComponentbyClass (Class|TempestBaseStateObject|GetPerformingActor) "/Script/TempestCombatFramework.TempestCombatComponent")) "(TagName=\"Status.Combat.InCombat\")")
            (Variables|Default|SetWalking%20Movement%20Speed (Variables|/Game/Integration/Properties/BP_GS_PlayerSpeedsPreoperty.BP_GS_PlayerSpeedsPreoperty_C|GetIn%20Combat%20Walking%20Movement%20Speed _asbp_gs_player_speeds_preoperty))
            (else
              (Variables|Default|SetWalking%20Movement%20Speed (Variables|/TempestCombatFramework/BehaviorProperties/BP_PlayerSpeedsProperty.BP_PlayerSpeedsProperty_C|GetWalking%20Movement%20Speed _asbp_gs_player_speeds_preoperty))))
          (return)))
      (return))))

(fn RotatetoTargetedActor
  (params (Alpha :type Float%20%28single-precision%29))
  (bind _currentperformingactor (Class|TempestBaseStateObject|GetPerformingActor))
  (bind _owner_character (Variables|Default|GetOwner%20Character))
  (bind _returnvalue (Actor|GetComponentbyClass _owner_character "/TempestCombatFramework/Components/BP_TempestTargetingComponent.BP_TempestTargetingComponent_C"))
  (bind _returnvalue_2 (Transformation|GetActorRotation _currentperformingactor))
  (bind (_roll _pitch) (Math|Rotator|BreakRotator _returnvalue_2))
  (Utilities|IsValid _returnvalue
    (:Is%20Valid
      (if (Class|TempestTargetingComponent|GetIsCurrentelyTargeting _returnvalue)
        (Transformation|SetActorRotation (Class|TempestBaseStateObject|GetPerformingActor) (Math|Rotator|MakeRotator _roll _pitch (.yaw (Math|Rotator|Lerp(Rotator) _returnvalue_2 (Math|Rotator|FindLookatRotation (Transformation|GetActorLocation _currentperformingactor) (Transformation|GetWorldLocation (Class|TempestBaseTargetingObject|GetTargetedComponent (Class|TempestTargetingComponent|GetCurrentActiveTargetingObject _returnvalue)))) Alpha true))))))))