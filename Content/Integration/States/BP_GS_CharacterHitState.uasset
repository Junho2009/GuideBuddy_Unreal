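; Tempest state-manager state for a character's hit reaction, shared by player and AI.
; On start it runs the selected ability and, for players not yet in combat, attaches weapons, sets InCombat status and updates the animation moveset.
; When deciding the next state, players go to Idle unchecked, while AI tries Turning, then randomly picks FollowTarget or Attack, with FollowTarget as Attack's fallback.
; Entry depends on whether its associated tagged abilities can run.
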(event EventStartState
  (bind _owner_character (Variables|Default|GetOwner%20Character))
  (bind _returnvalue (Actor|GetComponentbyClass _owner_character "/TempestCombatFramework/Components/BP_TempestBaseCombatComponent.BP_TempestBaseCombatComponent_C"))
  (|CallParentFunction)
  (Class|TempestBaseAbilityManagerComponent|PerformAbilityOfClass (Actor|GetComponentbyClass (Class|TempestBaseStateObject|GetPerformingActor) "/Script/TempestCombatFramework.TempestBaseAbilityManagerComponent") (CallFunction|GetSelectedAbility))
  (bind _returnvalue_2 (Class|TempestGeneralLibrary|GetIsPawnControlledbyPlayer (Variables|Default|GetOwner%20Character)))
  (if _returnvalue_2
    (if (not (GameplayTags|HasTag (Class|TempestCombatComponent|GetCombatStatus _returnvalue) "(TagName=\"Status.Combat.InCombat\")"))
      (Default|AttachAllWeapons (Default|GetEquippedWeapon _returnvalue) true)
      (Class|TempestCombatComponent|ModifyCombatStatus _returnvalue "(GameplayTags=((TagName=\"Status.Combat.InCombat\")))" "Add")
      (Class|BPITCFGeneralInterface|AssignMoveset(Message) (Components|SkeletalMesh|GetAnimInstance (Variables|/Script/Engine.Character|GetMesh _owner_character)) "NewEnumerator1"))))

(fn DecideNextState
  (bind _tempest_state_manager_component (CallFunction|GetTempestStateManagerComponent))
  (bind _tempest_state_manager_component_2 (CallFunction|GetTempestStateManagerComponent))
  (bind _tempest_state_manager_component_3 (CallFunction|GetTempestStateManagerComponent))
  (bind _tempest_state_manager_component_4 (CallFunction|GetTempestStateManagerComponent))
  (|CallParentFunction)
  (bind _returnvalue (Class|TempestGeneralLibrary|GetIsPawnControlledbyPlayer (Variables|Default|GetOwner%20Character)))
  (if _returnvalue
    (Class|TempestBaseStateManagerComponent|TryPerformStateOfClass _tempest_state_manager_component_2 (Utilities|GetClass (Class|TempestBaseStateManagerComponent|GetStateOfGameplayTag _tempest_state_manager_component_2 "(TagName=\"State.Idle\")")) false)
    (else
      (bind _returnvalue_2 (Class|TempestBaseStateManagerComponent|TryPerformStateOfClass _tempest_state_manager_component_3 (Utilities|GetClass (Class|TempestBaseStateManagerComponent|GetStateOfGameplayTag _tempest_state_manager_component_3 "(TagName=\"State.Turning\")")) true))
      (if (not _returnvalue_2)
        (if (Math|Random|RandomBool)
          (Class|TempestBaseStateManagerComponent|TryPerformStateOfClass _tempest_state_manager_component_4 (Utilities|GetClass (Class|TempestBaseStateManagerComponent|GetStateOfGameplayTag _tempest_state_manager_component_4 "(TagName=\"State.FollowTarget\")")) true :!label _label)
          (else
            (bind _returnvalue_3 (Class|TempestBaseStateManagerComponent|TryPerformStateOfClass _tempest_state_manager_component (Utilities|GetClass (Class|TempestBaseStateManagerComponent|GetStateOfGameplayTag _tempest_state_manager_component "(TagName=\"State.Attack\")")) true))
            (if (not _returnvalue_3)
              (goto _label))))))))

(fn CanPerformState
  (bind _return_value (CallFunction|CheckCanRunAssociatedAbilitiesOfTag "(TagName=\"List.One\")"))
  (return _return_value))