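; Enemy attacking state for the Tempest state manager, which runs the selected ability through the actor's ability manager on start.
; It can be performed only if an associated List.One ability can run and the owner is either player-controlled or has a valid combat target.
; When deciding the next state, it tries UnEquip, then Turning, then restarting itself, and finally falls back to FollowTarget.
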(event EventStartState
  (|CallParentFunction)
  (Class|TempestBaseAbilityManagerComponent|PerformAbilityOfClass (Actor|GetComponentbyClass (Class|TempestBaseStateObject|GetPerformingActor) "/Script/TempestCombatFramework.TempestBaseAbilityManagerComponent") (CallFunction|GetSelectedAbility)))

(fn DecideNextState
  (bind _tempest_state_manager_component (CallFunction|GetTempestStateManagerComponent))
  (bind _tempest_state_manager_component_2 (CallFunction|GetTempestStateManagerComponent))
  (bind _tempest_state_manager_component_3 (CallFunction|GetTempestStateManagerComponent))
  (|CallParentFunction)
  (bind _returnvalue (Class|TempestBaseStateManagerComponent|TryPerformStateOfClass _tempest_state_manager_component_2 (Utilities|GetClass (Class|TempestBaseStateManagerComponent|GetStateOfGameplayTag _tempest_state_manager_component_2 "(TagName=\"State.UnEquip\")")) true))
  (if (not _returnvalue)
    (bind _returnvalue_2 (Class|TempestBaseStateManagerComponent|TryPerformStateOfClass _tempest_state_manager_component_3 (Utilities|GetClass (Class|TempestBaseStateManagerComponent|GetStateOfGameplayTag _tempest_state_manager_component_3 "(TagName=\"State.Turning\")")) true))
    (if (not _returnvalue_2)
      (bind _returnvalue_3 (Class|TempestBaseStateObject|RestartState true))
      (if (not _returnvalue_3)
        (Class|TempestBaseStateManagerComponent|TryPerformStateOfClass _tempest_state_manager_component (Utilities|GetClass (Class|TempestBaseStateManagerComponent|GetStateOfGameplayTag _tempest_state_manager_component "(TagName=\"State.FollowTarget\")")) true)))))

(fn CanPerformState
  (bind _return_value (CallFunction|CheckCanRunAssociatedAbilitiesOfTag "(TagName=\"List.One\")"))
  (if _return_value
    (bind _returnvalue (Class|TempestGeneralLibrary|GetIsPawnControlledbyPlayer (Variables|Default|GetOwner%20Character)))
    (if _returnvalue
      _
      (else
        (Utilities|IsValid (Class|TempestCombatComponent|GetCombatTarget (Actor|GetComponentbyClass (Class|TempestBaseStateObject|GetPerformingActor) "/TempestCombatFramework/Components/BP_TempestBaseCombatComponent.BP_TempestBaseCombatComponent_C"))
          (:Is%20Valid
            _)
          (:Is%20Not%20Valid
            (return false)))))
    (return true)
    (else
      (return false))))