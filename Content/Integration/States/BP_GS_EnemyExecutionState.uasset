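; Enemy execution state for the Tempest state manager that performs its selected ability on the performing actor when started.
; Entry is gated on the abilities associated with the List.One tag being runnable.
; On construction, a looping half-second timer repeatedly attempts a state restart, clearing itself once the performing actor is invalid.
; Deciding the next state attempts a condition-checked switch to the UnEquip state, looked up by gameplay tag.
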(event Custom|CanExecute
  (Utilities|IsValid (Class|TempestBaseStateObject|GetPerformingActor)
    (:Is%20Valid
      (Class|TempestBaseStateObject|RestartState true))
    (:Is%20Not%20Valid
      (Utilities|Time|ClearTimerbyFunctionName 0 "CanExecute"))))

(event EventStartState
  (|CallParentFunction)
  (Class|TempestBaseAbilityManagerComponent|PerformAbilityOfClass (Actor|GetComponentbyClass (Class|TempestBaseStateObject|GetPerformingActor) "/Script/TempestCombatFramework.TempestBaseAbilityManagerComponent") (CallFunction|GetSelectedAbility)))

(event EventConstructState
  (|CallParentFunction)
  (Utilities|Time|SetTimerbyFunctionName 0 "CanExecute" 0.5 true))

(fn CanPerformState
  (bind _return_value (CallFunction|CheckCanRunAssociatedAbilitiesOfTag "(TagName=\"List.One\")"))
  (return _return_value))

(fn DecideNextState
  (bind _tempest_state_manager_component (CallFunction|GetTempestStateManagerComponent))
  (|CallParentFunction)
  (Class|TempestBaseStateManagerComponent|TryPerformStateOfClass _tempest_state_manager_component (Utilities|GetClass (Class|TempestBaseStateManagerComponent|GetStateOfGameplayTag _tempest_state_manager_component "(TagName=\"State.UnEquip\")")) true))