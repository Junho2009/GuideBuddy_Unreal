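; Player katana-and-scabbard weapon that shows the player health/posture widget while equipped and removes it on unequip.
; Update Meshes attaches both meshes to the owner's skeletal mesh and registers their equip sockets; only the katana changes socket when drawn.
; Update Traces builds multi-sphere traces through the owner's Tempest collision manager, tagged for the sword blade and a kick socket on the body.
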(event EventEquipWeapon
  (|CallParentFunction)
  (bind _returnvalue (UserInterface|CreateWidget "/Game/Integration/Widgets/WB_PlayerHealthPosture.WB_PlayerHealthPosture_C" (Game|GetPlayerController 0) (Game|GetPlayerCharacter 0)))
  (bind _output_get (Variables|Default|SetPlayer%20Health _returnvalue))
  (UserInterface|Viewport|AddtoViewport _output_get 0))

(event EventUnEquipWeapon
  (Widget|RemovefromParent (Variables|Default|GetPlayer%20Health))
  (|CallParentFunction))

(fn ConstructionScript
  (|CallParentFunction))

(fn UpdateMeshes
  (bind _returnvalue (Components|GetOwner))
  (bind _returnvalue_2 (Actor|GetComponentbyClass _returnvalue "/Script/Engine.SkeletalMeshComponent"))
  ;[1 1 1] This Represents Weapon 0
  (bind _returnvalue_3 (AddComponent|AddStaticMeshComponent false))
  (CallFunction|RegisterWeapon (Utilities|Struct|MakeS_WeaponDetails _returnvalue_3 "Scabbard_Target01" "Scabbard_Target01"))
  (Transformation|AttachComponentToComponent _returnvalue_3 _returnvalue_2 "Scabbard_Target01" "SnapToTarget" "SnapToTarget" "KeepWorld" true)
  ;[1 1 1] This Represents Weapon 1
  (bind _returnvalue_4 (AddComponent|AddStaticMeshComponent false))
  (CallFunction|RegisterWeapon (Utilities|Struct|MakeS_WeaponDetails _returnvalue_4 "katana_r" "katana_Targer01"))
  (Transformation|AttachComponentToComponent _returnvalue_4 _returnvalue_2 "katana_Targer01" "SnapToTarget" "SnapToTarget" "KeepWorld" true))

(fn UpdateTraces
  (bind _returnvalue (Components|GetOwner))
  (bind _createdtraceobject (Class|TempestCollisionManagerComponent|ConstructTraceOfClass (Actor|GetComponentbyClass (Components|GetOwner) "/TempestCombatFramework/Components/BP_TempestCollisionManager.BP_TempestCollisionManager_C") "/TempestCombatFramework/Trace/BP_BaseMultiSphereTraceObject.BP_BaseMultiSphereTraceObject_C"))
  (Variables|/Script/TempestCombatFramework.TempestBaseTraceObject|SetTraceGameplayTag _createdtraceobject "(TagName=\"Trace.Right Hand Weapon\")")
  (Class|TempestBaseTraceObject|SetTraceMeshInfo _createdtraceobject (.WeaponMesh (Utilities|Struct|BreakS_WeaponDetails (Utilities|Array|Get(acopy) (CallFunction|GetWeaponProperties) 1))) (Utilities|Array|MakeArray "Weapon Trace 1" "Weapon Trace 2" "Weapon Trace 3" "Weapon Trace 4" "Weapon Trace 5"))
  (bind _createdtraceobject_2 (Class|TempestCollisionManagerComponent|ConstructTraceOfClass (Actor|GetComponentbyClass _returnvalue "/TempestCombatFramework/Components/BP_TempestCollisionManager.BP_TempestCollisionManager_C") "/TempestCombatFramework/Trace/BP_BaseMultiSphereTraceObject.BP_BaseMultiSphereTraceObject_C"))
  (Variables|/Script/TempestCombatFramework.TempestBaseTraceObject|SetTraceGameplayTag _createdtraceobject_2 "(TagName=\"Trace.Kick\")")
  (Class|TempestBaseTraceObject|SetTraceMeshInfo _createdtraceobject_2 (Actor|GetComponentbyClass _returnvalue "/Script/Engine.SkeletalMeshComponent") (Utilities|Array|MakeArray "Kick Trace")))