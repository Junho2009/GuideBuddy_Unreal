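; BP_GS_TryPerformAbilitiesOfGameplayTag is a special property that makes its owning character try abilities identified by a list of gameplay tags.
; When processed with valid input, it resolves each tag to an ability class through the Tempest ability manager component and stops at the first one performed successfully, with condition checks on.
; Its can-process check returns true if any tagged ability can currently be performed by the owner.
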(event EventProcessSpecialProperty
  (Utilities|IsValid (Class|TempestInputBufferProperty|GetInputtoProcess)
    (:Is%20Valid
      (bind _ascharacter (Utilities|Casting|CastToCharacter (Class|TempestSpecialProperty|GetPropertyOwner)))
      (bind _array_element (Utilities|Array|ForEachLoopwithBreak (Variables|Default|GetAbility%20Tags) :!label _label)
        (:LoopBody
          (bind _returnvalue (Class|TempestBaseAbilityManagerComponent|TryPerformAbilityOfClass (Actor|GetComponentbyClass _ascharacter "/Script/TempestCombatFramework.TempestBaseAbilityManagerComponent") (Utilities|GetClass (Class|TempestBaseAbilityManagerComponent|GetAbilityOfGameplayTag (Actor|GetComponentbyClass _ascharacter "/Script/TempestCombatFramework.TempestBaseAbilityManagerComponent") _array_element)) true))
          (if _returnvalue
            (goto _label Break)))))))

(fn GetCanProcessProperty
  (bind _asactor (Utilities|Casting|CastToActor (Class|TempestSpecialProperty|GetPropertyOwner)))
  (for _array_element (Variables|Default|GetAbility%20Tags)
    (if (Class|TempestBaseAbilityManagerComponent|GetCanPerformAbilityOfClass (Actor|GetComponentbyClass _asactor "/Script/TempestCombatFramework.TempestBaseAbilityManagerComponent") (Utilities|GetClass (Class|TempestBaseAbilityManagerComponent|GetAbilityOfGameplayTag (Actor|GetComponentbyClass _asactor "/Script/TempestCombatFramework.TempestBaseAbilityManagerComponent") _array_element)))
      (return (Class|TempestBaseAbilityManagerComponent|GetCanPerformAbilityOfClass (Actor|GetComponentbyClass _asactor "/Script/TempestCombatFramework.TempestBaseAbilityManagerComponent") (Utilities|GetClass (Class|TempestBaseAbilityManagerComponent|GetAbilityOfGameplayTag (Actor|GetComponentbyClass _asactor "/Script/TempestCombatFramework.TempestBaseAbilityManagerComponent") _array_element))))))
  (return false))