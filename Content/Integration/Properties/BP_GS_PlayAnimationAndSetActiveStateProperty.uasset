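; Special property that plays an animation montage on its owning Character and switches that character's active Tempest state.
; On processing, if the input to process is valid, it plays the montage and passes the state matching StateGameplayTag to the Tempest state manager component.
; It reports itself processable only when the ability manager has an active ability and both the montage and tag are valid.
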(event EventProcessSpecialProperty
  (Utilities|IsValid (Class|TempestInputBufferProperty|GetInputtoProcess)
    (:Is%20Valid
      (bind _ascharacter (Utilities|Casting|CastToCharacter (Class|TempestSpecialProperty|GetPropertyOwner)))
      (Animation|PlayAnimMontage _ascharacter (Variables|Default|GetAnim%20Montage) 1.0 "None")
      (Class|TempestBaseStateManagerComponent|SetCurrentActiveState (Actor|GetComponentbyClass _ascharacter "/Script/TempestCombatFramework.TempestBaseStateManagerComponent") (Class|TempestBaseStateManagerComponent|GetStateOfGameplayTag (Actor|GetComponentbyClass _ascharacter "/Script/TempestCombatFramework.TempestBaseStateManagerComponent") (Variables|Default|GetState%20Gameplay%20Tag))))))

(fn GetCanProcessProperty
  (bind _ascharacter (Utilities|Casting|CastToCharacter (Class|TempestSpecialProperty|GetPropertyOwner)))
  (return (Math|Boolean|ANDBoolean (Utilities|IsValid (Class|TempestBaseAbilityManagerComponent|GetCurrentActiveAbility (Actor|GetComponentbyClass _ascharacter "/Script/TempestCombatFramework.TempestBaseAbilityManagerComponent"))) (Utilities|IsValid (Variables|Default|GetAnim%20Montage)) (GameplayTags|IsGameplayTagValid (Variables|Default|GetState%20Gameplay%20Tag)))))