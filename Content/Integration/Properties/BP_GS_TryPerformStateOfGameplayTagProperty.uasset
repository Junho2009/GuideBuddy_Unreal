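; Input-driven special property that makes its owning Character perform the state matching a configured gameplay tag.
; The can-process check resolves the tag to a state class through the Character's TempestBaseStateManagerComponent and asks whether that state can be performed.
; When processed with a valid input, it optionally stops the current anim montage, then has the state manager perform that state class.
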(event EventProcessSpecialProperty
  (Utilities|IsValid (Class|TempestInputBufferProperty|GetInputtoProcess)
    (:Is%20Valid
      (bind _ascharacter (Utilities|Casting|CastToCharacter (Class|TempestSpecialProperty|GetPropertyOwner)))
      (if (Variables|Default|GetCancel%20Montage)
        (Animation|StopAnimMontage _ascharacter 0))
      (Class|TempestBaseStateManagerComponent|PerformStateOfClass (Actor|GetComponentbyClass _ascharacter "/Script/TempestCombatFramework.TempestBaseStateManagerComponent") (Utilities|GetClass (Class|TempestBaseStateManagerComponent|GetStateOfGameplayTag (Actor|GetComponentbyClass _ascharacter "/Script/TempestCombatFramework.TempestBaseStateManagerComponent") (Variables|Default|GetState%20Gameplay%20Tag)))))))

(fn GetCanProcessProperty
  (bind _ascharacter (Utilities|Casting|CastToCharacter (Class|TempestSpecialProperty|GetPropertyOwner)))
  (return (Class|TempestBaseStateManagerComponent|GetCanPerformStateOfClass (Actor|GetComponentbyClass _ascharacter "/Script/TempestCombatFramework.TempestBaseStateManagerComponent") (Utilities|GetClass (Class|TempestBaseStateManagerComponent|GetStateOfGameplayTag (Actor|GetComponentbyClass _ascharacter "/Script/TempestCombatFramework.TempestBaseStateManagerComponent") (Variables|Default|GetState%20Gameplay%20Tag))))))