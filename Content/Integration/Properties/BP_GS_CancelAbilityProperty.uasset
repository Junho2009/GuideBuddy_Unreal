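; Special property from the Tempest ability system that cancels its owning character's currently active ability.
; It can only be processed while the owner's ability manager component reports a valid active ability.
; When processed with a valid input to process, it optionally stops that ability's montage based on the CancelMontage flag, then cancels the ability.
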(event EventProcessSpecialProperty
  (Utilities|IsValid (Class|TempestInputBufferProperty|GetInputtoProcess)
    (:Is%20Valid
      (bind _ascharacter (Utilities|Casting|CastToCharacter (Class|TempestSpecialProperty|GetPropertyOwner)))
      (if (Variables|Default|GetCancel%20Montage)
        (Animation|StopAnimMontage _ascharacter (Class|TempestBaseAbilityObject|GetActiveAbilityMontage (Class|TempestBaseAbilityManagerComponent|GetCurrentActiveAbility (Actor|GetComponentbyClass _ascharacter "/Script/TempestCombatFramework.TempestBaseAbilityManagerComponent")))))
      (Class|TempestBaseAbilityObject|CancelAbility (Class|TempestBaseAbilityManagerComponent|GetCurrentActiveAbility (Actor|GetComponentbyClass _ascharacter "/Script/TempestCombatFramework.TempestBaseAbilityManagerComponent"))))))

(fn GetCanProcessProperty
  (bind _ascharacter (Utilities|Casting|CastToCharacter (Class|TempestSpecialProperty|GetPropertyOwner)))
  (return (Utilities|IsValid (Class|TempestBaseAbilityManagerComponent|GetCurrentActiveAbility (Actor|GetComponentbyClass _ascharacter "/Script/TempestCombatFramework.TempestBaseAbilityManagerComponent")))))