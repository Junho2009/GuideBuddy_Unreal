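; Player controller for the Tempest Combat Framework (TCF) GS setup that routes Enhanced Input into the controlled pawn's Tempest components.
; BeginPlay adds the GS mapping context, then records, binds and watch-lists its actions on the pawn's input component.
; Possess forces the idle state and refreshes input history, while UnPossess restores the pawn's default controller.
; Helpers expose movement input and yaw-relative direction; looking values return zero and spectator-camera toggling is unwired.
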(event EventPossess
  (params (PossessedPawn :type Pawn%20Object%20Reference))
  (bind _returnvalue (Actor|GetComponentbyClass PossessedPawn "/Script/TempestCombatFramework.TempestBaseStateManagerComponent"))
  (|CallParentFunction PossessedPawn)
  (Class|TempestBaseStateManagerComponent|PerformStateOfClass _returnvalue (Utilities|GetClass (Class|TempestBaseStateManagerComponent|GetStateOfGameplayTag _returnvalue "(TagName=\"State.Idle\")")))
  (Class|TempestBaseInputComponent|RefreshInputHistory (Actor|GetComponentbyClass (Pawn|GetControlledPawn) "/Script/TempestCombatFramework.TempestBaseInputComponent")))

(event EventUnPossess
  (params (UnpossessedPawn :type Pawn%20Object%20Reference))
  (|CallParentFunction UnpossessedPawn)
  (Pawn|SpawnDefaultController UnpossessedPawn))

(event EventBeginPlay
  (|CallParentFunction)
  (Input|AddMappingContext (PlayerController|LocalPlayerSubsystems|GetEnhancedInputLocalPlayerSubsystem) "/Game/Integration/GS_Player_InputMappings.GS_Player_InputMappings" 0 "(bIgnoreAllPressedKeysUntilRelease=True,bForceImmediately=False,bNotifyUserSettings=False)")
  (CallFunction|UpdateInputComponent "/Game/Integration/GS_Player_InputMappings.GS_Player_InputMappings"))

(event Input|KeyboardEvents|N
  (params (Key :type Key%20Structure :default "None")))

(fn ConstructionScript)

(fn UpdateInputComponent
  (params (InMappingContext :type Input%20Mapping%20Context%20Object%20Reference))
  (bind _returnvalue (Pawn|GetControlledPawn))
  (bind _returnvalue_2 (Actor|GetComponentbyClass _returnvalue "/Script/TempestCombatFramework.TempestBaseInputComponent"))
  (Class|TempestBaseInputComponent|SetRecordedMappingContexts _returnvalue_2 InMappingContext "(TagName=\"List.One\")")
  (bind _returnvalue_3 (Class|TempestGeneralLibrary|GetInputsOfInputContext InMappingContext))
  (Class|TempestBaseInputComponent|CreateBindingsforInputActions _returnvalue_2 _returnvalue_3)
  (Class|TempestBaseInputComponent|AddInputstoWatchListTag _returnvalue_2 _returnvalue_3 "(TagName=\"List.One\")"))

(fn GetDirectionfromMovementInputs
  (bind _returnvalue (Pawn|GetControlledPawn))
  (bind _returnvalue_2 (Pawn|GetControlRotation _returnvalue :!class /Script/Engine.Pawn))
  (bind _yaw (Math|Rotator|BreakRotator _returnvalue_2))
  (bind _returnvalue_3 (Math|Rotator|MakeRotator 0.0 0.0 _yaw))
  (return (Math|Vector|Normalize (+ (* (Math|Vector|GetRightVector _returnvalue_3) (Input|EnhancedActionValues|GetMoveRightLeft_Input)) (* (Math|Vector|GetForwardVector _returnvalue_3) (Input|EnhancedActionValues|GetMoveForwardBackward_Input))))))

(fn GetLookingValues
  (return 0.0 0.0))

(fn GetMovementInputs
  (return (Input|EnhancedActionValues|GetMoveForwardBackward_Input) (Input|EnhancedActionValues|GetMoveRightLeft_Input)))