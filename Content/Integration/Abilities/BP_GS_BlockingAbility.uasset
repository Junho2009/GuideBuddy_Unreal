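; Blocking ability for the Tempest combat framework that plays a random block montage from the tagged montage list when started.
; It can run only outside death, parried and deflect states, while combat status carries the NoBlockTrigger tag.
; It also requires the combat target to be close and within a frontal cone, and refuses if already active or during a normal deflect.
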(event EventStartAbility
  (|CallParentFunction)
  (bind _list_of_montages (CallFunction|GetAbilityMontagesOfTag "(TagName=\"List.One\")"))
  (Variables|Default|SetBlocking%20Montages _list_of_montages)
  (CallFunction|PlayAbilityMontage (.OutItem (Utilities|Array|Random (Variables|Default|GetBlocking%20Montages))) 1.0 "MontageLength" 0.0 "None" true))

(fn CanPerformAbility
  (bind _returnvalue (CallFunction|GetIsCurrentAbilityActive))
  (bind _currentperformingactor (Class|TempestBaseAbilityObject|GetPerformingActor))
  (bind _currentperformingactor_2 (Class|TempestBaseAbilityObject|GetPerformingActor))
  (bind _currentperformingactor_3 (Class|TempestBaseAbilityObject|GetPerformingActor))
  (bind _tempestabilitycomponent (CallFunction|GetTempestAbilityComponent))
  (bind _returnvalue_2 (Class|TempestBaseAbilityManagerComponent|GetCurrentActiveAbility _tempestabilitycomponent))
  (bind _returnvalue_3 (Actor|GetComponentbyClass _currentperformingactor_3 "/Script/TempestCombatFramework.TempestBaseStateManagerComponent"))
  (bind _returnvalue_4 (not _returnvalue))
  (bind _returnvalue_5 (Class|TempestBaseStateManagerComponent|GetCurrentActiveState _returnvalue_3))
  (bind _stategameplaytag (Variables|/Script/TempestCombatFramework.TempestBaseStateObject|GetStateGameplayTag _returnvalue_5))
  (if (Math|Boolean|ANDBoolean (!= _stategameplaytag "(TagName=\"State.Death\")") (!= _stategameplaytag "(TagName=\"State.Parried\")") (!= _stategameplaytag "(TagName=\"State.Deflect\")") (GameplayTags|HasTag (Class|TempestCombatComponent|GetCombatStatus (Actor|GetComponentbyClass _currentperformingactor_3 "/Script/TempestCombatFramework.TempestCombatComponent")) "(TagName=\"Status.Combat.No Block Trigger\")"))
    (bind _returnvalue_6 (Class|TempestMathLibrary|GetDistanceBetweenActors _currentperformingactor (Class|TempestCombatComponent|GetCombatTarget (Actor|GetComponentbyClass _currentperformingactor "/Script/TempestCombatFramework.TempestCombatComponent"))))
    (bind _returnvalue_7 (Class|TempestMathLibrary|GetAnglesBetweenActors _currentperformingactor_2 (Class|TempestCombatComponent|GetCombatTarget (Actor|GetComponentbyClass _currentperformingactor_2 "/Script/TempestCombatFramework.TempestCombatComponent"))))
    (Utilities|IsValid _returnvalue_2
      (:Is%20Valid
        (return (Math|Boolean|ANDBoolean (Math|Float|InRange(Float) (.yaw _returnvalue_7) -6e+01 6e+01) (Math|Float|InRange(Float) _returnvalue_6 0.0 3.5e+02) _returnvalue_4 (!= (Variables|/Script/TempestCombatFramework.TempestBaseAbilityObject|GetAbilityGameplayTag _returnvalue_2) "(TagName=\"Ability.Deflect.Normal\")"))))
      (:Is%20Not%20Valid
        (return (Math|Boolean|ANDBoolean (Math|Float|InRange(Float) (.yaw _returnvalue_7) -6e+01 6e+01) (Math|Float|InRange(Float) _returnvalue_6 0.0 3.5e+02) _returnvalue_4))))
    (else
      (return false))))