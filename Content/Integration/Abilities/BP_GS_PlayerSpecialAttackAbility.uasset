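; Player special attack ability that starts its cooldown and plays a random montage from the set tagged List.One.
; It can only run while the special attack input is triggered, the combat component reports InCombat, a weapon is equipped and the cooldown is over.
; Cancelling ends the ability, and the remaining functions, such as projectile, strafing and incoming attack handling, are empty stubs returning defaults.
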(event EventStartAbility
  (|CallParentFunction)
  (Class|TempestBaseAbilityObject|ApplyAbilityCooldown)
  (bind _list_of_montages (CallFunction|GetAbilityMontagesOfTag "(TagName=\"List.One\")"))
  (CallFunction|PlayAbilityMontage (.OutItem (Utilities|Array|Random _list_of_montages)) 1.0 "Duration" 0.0 "None" true))

(event EventCancelAbility
  (|CallParentFunction)
  (Class|TempestBaseAbilityObject|EndAbility))

(fn CanPerformAbility
  (bind _currentperformingactor (Class|TempestBaseAbilityObject|GetPerformingActor))
  (bind _returnvalue (Actor|GetComponentbyClass _currentperformingactor "/TempestCombatFramework/Components/BP_TempestBaseCombatComponent.BP_TempestBaseCombatComponent_C"))
  (if (Utilities|Enum|Equal(Enum) (Class|TempestBaseInputComponent|GetInputActionCurrentTriggerEvent (Actor|GetComponentbyClass (Class|TempestBaseAbilityObject|GetPerformingActor) "/Script/TempestCombatFramework.TempestBaseInputComponent") "/TempestCombatFramework/Input/SpecialAttack_Input.SpecialAttack_Input") "Triggered")
    (return (Math|Boolean|ANDBoolean (GameplayTags|HasTag (Class|TempestCombatComponent|GetCombatStatus _returnvalue) "(TagName=\"Status.Combat.InCombat\")") (Utilities|IsValid (Default|GetEquippedWeapon _returnvalue)) (not (Class|TempestBaseAbilityObject|GetIsAbilityonCooldown))))
    (else
      (return false))))

(fn GetAbilityProjectile
  (return 0))

(fn GetAssociatedPassiveAbilities
  (return 0))

(fn GetBlockTimeSinceLastClicked
  (return 0.0))

(fn GetMontageCounterforAbility
  (return 0))

(fn GetMontageOfGameplayTag
  (params (Montage%20Tag :type Gameplay%20Tag%20Structure))
  (return 0))

(fn GetStrafingValues
  (return 0.0 "0, 0, 0"))

(fn ProcessIncomingAttack
  (params (Incoming%20Attack%20Type :type Gameplay%20Tag%20Structure))
  (return false))