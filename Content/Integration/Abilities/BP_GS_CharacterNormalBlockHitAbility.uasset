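; Gameplay ability that plays a character's reaction to a hit landing on their normal block.
; It picks the block montage from the incoming attack's swing direction, falling back to random, then applies the weapon's block impact effect and registers for ticking.
; CanPerformAbility requires a roughly frontal angle: AI checks blocking state against its combat target, while players check attacker, combat status, non-grab attacks and block state or input timing.
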(event EventStartAbility
  (bind _currentperformingactor (Class|TempestBaseAbilityObject|GetPerformingActor))
  (bind _returnvalue (Actor|GetComponentbyClass _currentperformingactor "/TempestCombatFramework/Components/BP_TempestBaseCombatComponent.BP_TempestBaseCombatComponent_C"))
  (|CallParentFunction)
  (bind _list_of_montages (CallFunction|GetAbilityMontagesOfTag "(TagName=\"List.One\")"))
  (Variables|Default|SetBlocked%20Montages _list_of_montages)
  (bind _asbp_normal_attack_property (Utilities|Casting|CastToBP_NormalAttackProperty (Variables|/Script/TempestCombatFramework.TempestCombatComponent|GetReceivedAttackProperty (Actor|GetComponentbyClass (Class|TempestBaseAbilityObject|GetPerformingActor) "/Script/TempestCombatFramework.TempestCombatComponent")))
    (:then
      (switch Utilities|FlowControl|Switch|SwitchonE_SwingDirection (Variables|/TempestCombatFramework/AttackProperties/BP_NormalAttackProperty.BP_NormalAttackProperty_C|GetSwing%20Direction _asbp_normal_attack_property)
        (:NewEnumerator3
          (CallFunction|PlayAbilityMontage (Utilities|Array|Get(acopy) (Variables|Default|GetBlocked%20Montages)) 1.0 "MontageLength" 0.0 "None" true :!label _label))
        (:NewEnumerator5
          (goto _label))
        (:NewEnumerator8
          (goto _label))
        (:NewEnumerator9
          (CallFunction|PlayAbilityMontage (Utilities|Array|Get(acopy) (Variables|Default|GetBlocked%20Montages) 1) 1.0 "MontageLength" 0.0 "None" true :!label _label_2))
        (:NewEnumerator10
          (goto _label))
        (:NewEnumerator11
          (goto _label))
        (:NewEnumerator12
          (goto _label_2))
        (:NewEnumerator13
          (goto _label_2))))
    (:CastFailed
      (CallFunction|PlayAbilityMontage (.OutItem (Utilities|Array|Random (Variables|Default|GetBlocked%20Montages))) 1.0 "MontageLength" 0.0 "None" true)))
  (bind _found_impact_effect (Default|GetImpactEffectClassOfTag (Variables|/TempestCombatFramework/Actors/Weapons/BP_BaseWeapon.BP_BaseWeapon_C|GetData%20Asset%20Info%20Reference (Default|GetEquippedWeapon _returnvalue)) "(TagName=\"Impact.Effect.Block\")"))
  (Class|TempestDefensePropertiesObject|ApplyHitEffectOfClass (Variables|/Script/TempestCombatFramework.TempestCombatComponent|GetOwnerDefenseProperty _returnvalue) _found_impact_effect)
  (Class|TempestTickingComponent|AddTickableObject (Actor|GetComponentbyClass (Class|TempestBaseAbilityObject|GetPerformingActor) "/Script/TempestCore.TempestTickingComponent") self))

(event EventCancelAbility
  (|CallParentFunction)
  (Class|TempestBaseAbilityObject|EndAbility))

(event EventEndAbility
  (|CallParentFunction)
  (Class|TempestTickingComponent|RemoveTickableObject (Actor|GetComponentbyClass (Class|TempestBaseAbilityObject|GetPerformingActor) "/Script/TempestCore.TempestTickingComponent") self))

(fn CanPerformAbility
  (bind _currentperformingactor (Class|TempestBaseAbilityObject|GetPerformingActor))
  (bind _currentperformingactor_2 (Class|TempestBaseAbilityObject|GetPerformingActor))
  (bind _currentperformingactor_3 (Class|TempestBaseAbilityObject|GetPerformingActor))
  (bind _owner_character (Variables|Default|GetOwner%20Character))
  (bind _owner_character_2 (Variables|Default|GetOwner%20Character))
  (bind _returnvalue (Actor|GetComponentbyClass _owner_character "/TempestCombatFramework/Components/BP_TempestBaseCombatComponent.BP_TempestBaseCombatComponent_C"))
  (bind _returnvalue_2 (Actor|GetComponentbyClass _currentperformingactor_2 "/Script/TempestCombatFramework.TempestBaseStateManagerComponent"))
  (bind _returnvalue_3 (Actor|GetComponentbyClass _owner_character_2 "/Script/TempestCombatFramework.TempestBaseStateManagerComponent"))
  (bind _returnvalue_4 (Actor|GetComponentbyClass _currentperformingactor "/Script/TempestCombatFramework.TempestBaseInputComponent"))
  (bind _returnvalue_5 (Class|TempestBaseStateManagerComponent|GetCurrentActiveState _returnvalue_2))
  (bind _returnvalue_6 (Class|TempestBaseStateManagerComponent|GetCurrentActiveState _returnvalue_3))
  (bind _returnvalue_7 (Class|TempestBaseInputComponent|GetInputActionCurrentTriggerEvent _returnvalue_4 "/TempestCombatFramework/Input/RightMouse_Input.RightMouse_Input"))
  (bind _receivedattackproperty (Variables|/Script/TempestCombatFramework.TempestCombatComponent|GetReceivedAttackProperty _returnvalue))
  (bind _returnvalue_8 (Utilities|Enum|Equal(Enum) _returnvalue_7 "Triggered"))
  (bind _stategameplaytag (Variables|/Script/TempestCombatFramework.TempestBaseStateObject|GetStateGameplayTag _returnvalue_6))
  (bind _stategameplaytag_2 (Variables|/Script/TempestCombatFramework.TempestBaseStateObject|GetStateGameplayTag _returnvalue_5))
  (bind _returnvalue_9 (Class|TempestGeneralLibrary|GetIsPawnControlledbyPlayer (Variables|Default|GetOwner%20Character)))
  (if (not _returnvalue_9)
    (if (and (!= _stategameplaytag_2 "(TagName=\"State.Death\")") (or (== _stategameplaytag_2 "(TagName=\"State.Trying To Block\")") (CallFunction|GetIsCurrentAbilityActive)))
      (bind _returnvalue_10 (Class|TempestMathLibrary|GetAnglesBetweenActors _currentperformingactor_3 (Class|TempestCombatComponent|GetCombatTarget (Actor|GetComponentbyClass _currentperformingactor_3 "/Script/TempestCombatFramework.TempestCombatComponent"))))
      (return (Math|Float|InRange(Float) (.yaw _returnvalue_10) -65.0 65.0))
      (else
        (return false)))
    (else
      (Utilities|IsValid (Class|TempestBaseStateManagerComponent|GetCurrentActiveState _returnvalue_3)
        (:Is%20Valid
          (bind _returnvalue_11 (Class|TempestMathLibrary|GetAnglesBetweenActors (Variables|Default|GetOwner%20Character) (Class|TempestAttackPropertiesObject|GetAttackPropertyOwner _receivedattackproperty)))
          (bind _return_value (Class|BPITempestAbilitiesandStates|GetBlockTimeSinceLastClicked(Message) (Class|TempestBaseStateManagerComponent|GetStateOfGameplayTag (Actor|GetComponentbyClass (Variables|Default|GetOwner%20Character) "/Script/TempestCombatFramework.TempestBaseStateManagerComponent") "(TagName=\"State.Normal Block\")")))
          (return (Math|Boolean|ANDBoolean (!= (Variables|/Script/TempestCombatFramework.TempestAttackPropertiesObject|GetAttackPropertyTag _receivedattackproperty) "(TagName=\"Property.Attack.Grab\")") (Math|Float|InRange(Float) (.yaw _returnvalue_11) -65.0 65.0) (or (and (not _returnvalue_8) (Math|Float|InRange(Float) _return_value 0.15 0.25)) (Math|Boolean|ORBoolean (== _stategameplaytag "(TagName=\"State.Normal Block\")") (and (== _stategameplaytag "(TagName=\"State.Deflect\")") _returnvalue_8) (CallFunction|GetIsCurrentAbilityActive))) (GameplayTags|HasTag (Class|TempestCombatComponent|GetCombatStatus _returnvalue) "(TagName=\"Status.Combat.InCombat\")"))))
        (:Is%20Not%20Valid
          (return false))))))

(fn AnyMontageIsPlaying?
  (for _array_element (Variables|Default|GetBlocked%20Montages)
    (if (Animation|Montage|MontageIsPlaying (Components|SkeletalMesh|GetAnimInstance (Variables|/Script/Engine.Character|GetMesh (Variables|Default|GetOwner%20Character))) _array_element)
      (return (Animation|Montage|MontageIsPlaying (Components|SkeletalMesh|GetAnimInstance (Variables|/Script/Engine.Character|GetMesh (Variables|Default|GetOwner%20Character))) _array_element))))
  (return false))