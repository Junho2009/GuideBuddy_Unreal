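; BP_GS_CharacterKnockHitAbility is a character ability that plays a knock hit reaction when the performer receives a Leap attack.
; It can run only if the performer is not invincible, has an equipped weapon and the ability is off cooldown.
; On start it plays a random tagged montage, then applies the default impact effect from the performer's own weapon data through its defense property.
; Cancelling ends the ability.
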(event EventStartAbility
  (bind _currentperformingactor (Class|TempestBaseAbilityObject|GetPerformingActor))
  (bind _returnvalue (Actor|GetComponentbyClass _currentperformingactor "/TempestCombatFramework/Components/BP_TempestBaseCombatComponent.BP_TempestBaseCombatComponent_C"))
  (|CallParentFunction)
  (bind _list_of_montages (CallFunction|GetAbilityMontagesOfTag "(TagName=\"List.One\")"))
  (bind _output_get (Variables|Default|SetHit%20Reaction%20Montages _list_of_montages))
  (CallFunction|PlayAbilityMontage (.OutItem (Utilities|Array|Random _output_get)) 1.0 "MontageLength" 0.0 "None" true)
  (bind _found_impact_effect (Default|GetImpactEffectClassOfTag (Variables|/TempestCombatFramework/Actors/Weapons/BP_BaseWeapon.BP_BaseWeapon_C|GetData%20Asset%20Info%20Reference (Default|GetEquippedWeapon _returnvalue)) "(TagName=\"Impact.Effect.Default\")"))
  (Class|TempestDefensePropertiesObject|ApplyHitEffectOfClass (Variables|/Script/TempestCombatFramework.TempestCombatComponent|GetOwnerDefenseProperty _returnvalue) _found_impact_effect))

(event EventCancelAbility
  (|CallParentFunction)
  (Class|TempestBaseAbilityObject|EndAbility))

(fn CanPerformAbility
  (bind _currentperformingactor (Class|TempestBaseAbilityObject|GetPerformingActor))
  (bind _returnvalue (Actor|GetComponentbyClass _currentperformingactor "/TempestCombatFramework/Components/BP_TempestBaseCombatComponent.BP_TempestBaseCombatComponent_C"))
  (if (not (GameplayTags|HasTag (Class|TempestCombatComponent|GetCombatStatus _returnvalue) "(TagName=\"Status.Combat.Invincible\")"))
    (return (Math|Boolean|ANDBoolean (== (Variables|/Script/TempestCombatFramework.TempestAttackPropertiesObject|GetAttackPropertyTag (Variables|/Script/TempestCombatFramework.TempestCombatComponent|GetReceivedAttackProperty _returnvalue)) "(TagName=\"Property.Attack.Leap\")") (not (Class|TempestBaseAbilityObject|GetIsAbilityonCooldown)) (Utilities|IsValid (Default|GetEquippedWeapon (Actor|GetComponentbyClass (Class|TempestBaseAbilityObject|GetPerformingActor) "/TempestCombatFramework/Components/BP_TempestBaseCombatComponent.BP_TempestBaseCombatComponent_C")))))
    (else
      (return false))))