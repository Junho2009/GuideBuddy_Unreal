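; Tempest ability that performs a paired execution on the performer's combat target when it is prone to riposte.
; The target's execution behavior property supplies montage pairs, choosing the first whose cached owner-target condition passes or is unset.
; It plays the attacker montage, passes the victim montage to the target's Executed ability, and triggers its Executed state.
; A syncing object constructed from the chosen entry ticks through the ticking component.
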(event EventTickTempestObject
  (params (Value :type Float%20%28single-precision%29))
  (bind _syncing_object (Variables|Default|GetSyncing%20Object))
  (Utilities|IsValid _syncing_object
    (:Is%20Valid
      (Default|TickSyncingObject _syncing_object))))

(event EventStartAbility
  (bind _currentperformingactor (Class|TempestBaseAbilityObject|GetPerformingActor))
  (bind _returnvalue (Actor|GetComponentbyClass _currentperformingactor "/Script/TempestCombatFramework.TempestCombatComponent"))
  (bind _foundcombattarget (Class|TempestCombatComponent|GetCombatTarget _returnvalue))
  (bind _returnvalue_2 (Actor|GetComponentbyClass _foundcombattarget "/Script/TempestCombatFramework.TempestBaseStateManagerComponent"))
  (|CallParentFunction)
  (bind _found_assasination_property (CallFunction|GetExecutionProperty))
  (bind _output_get (Variables|Default|SetExecution%20Montage (.PlayerAssasinationMontage (Utilities|Struct|BreakS_AssasinationProperties _found_assasination_property))))
  (Utilities|IsValid _output_get
    (:Is%20Valid
      (CallFunction|PlayAbilityMontage (Variables|Default|GetExecution%20Montage) 1.0 "Duration" 0.0 "None" true)
      (Class|BPITempestAbilitiesandStates|SetTargetMontage(Message) (Class|TempestBaseAbilityManagerComponent|GetAbilityOfGameplayTag (Actor|GetComponentbyClass _foundcombattarget "/Script/TempestCombatFramework.TempestBaseAbilityManagerComponent") "(TagName=\"Ability.Executed\")") (.AIAssasinatedMontage (Utilities|Struct|BreakS_AssasinationProperties _found_assasination_property)))
      (Class|TempestBaseStateManagerComponent|PerformStateOfClass _returnvalue_2 (Utilities|GetClass (Class|TempestBaseStateManagerComponent|GetStateOfGameplayTag _returnvalue_2 "(TagName=\"State.Executed\")")))
      (bind _returnvalue_3 (Game|ConstructObjectfromClass (Variables|Default|GetOwner%20Character) (.SyncingObject (Utilities|Struct|BreakS_AssasinationProperties _found_assasination_property)) (Class|TempestCombatComponent|GetCombatTarget (Actor|GetComponentbyClass (Class|TempestBaseAbilityObject|GetPerformingActor) "/Script/TempestCombatFramework.TempestCombatComponent"))))
      (bind _output_get_2 (Variables|Default|SetSyncing%20Object _returnvalue_3))
      (Default|ConstructSyncingObject _output_get_2)
      (Class|TempestTickingComponent|AddTickableObject (Actor|GetComponentbyClass (Class|TempestBaseAbilityObject|GetPerformingActor) "/Script/TempestCore.TempestTickingComponent") self))
    (:Is%20Not%20Valid
      (Class|TempestBaseAbilityObject|EndAbility))))

(fn CanPerformAbility
  (bind _currentperformingactor (Class|TempestBaseAbilityObject|GetPerformingActor))
  (bind _currentperformingactor_2 (Class|TempestBaseAbilityObject|GetPerformingActor))
  (bind _currentperformingactor_3 (Class|TempestBaseAbilityObject|GetPerformingActor))
  (bind _returnvalue (Actor|GetComponentbyClass _currentperformingactor_3 "/Script/TempestCombatFramework.TempestCombatComponent"))
  (bind _returnvalue_2 (Actor|GetComponentbyClass _currentperformingactor "/TempestCombatFramework/Components/BP_TempestBaseCombatComponent.BP_TempestBaseCombatComponent_C"))
  (bind _returnvalue_3 (Actor|GetComponentbyClass _currentperformingactor_2 "/Script/TempestCombatFramework.TempestBaseStateManagerComponent"))
  (bind _foundcombattarget (Class|TempestCombatComponent|GetCombatTarget _returnvalue))
  (bind _returnvalue_4 (Class|TempestBaseStateManagerComponent|GetCurrentActiveState _returnvalue_3))
  (bind _returnvalue_5 (Actor|GetComponentbyClass _foundcombattarget "/Script/TempestCombatFramework.TempestBaseStateManagerComponent"))
  (bind _stategameplaytag (Variables|/Script/TempestCombatFramework.TempestBaseStateObject|GetStateGameplayTag _returnvalue_4))
  (bind _returnvalue_6 (Class|TempestBaseStateManagerComponent|GetStateOfGameplayTag _returnvalue_5 "(TagName=\"State.Executed\")"))
  (Utilities|IsValid _returnvalue_4
    (:Is%20Valid
      (if (and (!= _stategameplaytag "(TagName=\"State.Death\")") (!= _stategameplaytag "(TagName=\"State.Attack\")"))
        (Utilities|IsValid _foundcombattarget
          (:Is%20Valid
            (if (GameplayTags|HasTag (Class|TempestCombatComponent|GetCombatStatus (Actor|GetComponentbyClass _foundcombattarget "/Script/TempestCombatFramework.TempestCombatComponent")) "(TagName=\"Status.Combat.Weakness.Prone To Riposte\")")
              (Utilities|IsValid _returnvalue_6
                (:Is%20Valid
                  (bind _found_assasination_property (CallFunction|GetExecutionProperty))
                  (return (Math|Boolean|ANDBoolean (Utilities|IsValid (Default|GetEquippedWeapon _returnvalue_2)) (GameplayTags|HasTag (Class|TempestCombatComponent|GetCombatStatus _returnvalue_2) "(TagName=\"Status.Combat.InCombat\")") (Class|TempestBaseStateObject|CanPerformState _returnvalue_6) (Utilities|IsValid (.PlayerAssasinationMontage (Utilities|Struct|BreakS_AssasinationProperties _found_assasination_property))) (Utilities|IsValid (.AIAssasinatedMontage (Utilities|Struct|BreakS_AssasinationProperties _found_assasination_property))))))
                (:Is%20Not%20Valid
                  (return false)))
              (else
                _)))
          (:Is%20Not%20Valid
            _))))
    (:Is%20Not%20Valid
      _))
  (return false))

(fn GetExecutionProperty
  (bind _currentperformingactor (Class|TempestBaseAbilityObject|GetPerformingActor))
  (bind _currentperformingactor_2 (Class|TempestBaseAbilityObject|GetPerformingActor))
  (bind _owner_character (Variables|Default|GetOwner%20Character))
  (bind _returnvalue (Actor|GetComponentbyClass _currentperformingactor "/Script/TempestCombatFramework.TempestCombatComponent"))
  (bind _returnvalue_2 (Actor|GetComponentbyClass _currentperformingactor_2 "/Script/TempestCombatFramework.TempestCombatComponent"))
  (bind _foundcombattarget (Class|TempestCombatComponent|GetCombatTarget _returnvalue_2))
  (bind _foundcombattarget_2 (Class|TempestCombatComponent|GetCombatTarget _returnvalue))
  (bind _returnvalue_3 (Actor|GetComponentbyClass _foundcombattarget "/TempestCombatFramework/Components/BP_TempestPropertiesComponent.BP_TempestPropertiesComponent_C"))
  (Utilities|IsValid _returnvalue_3
    (:Is%20Valid
      (bind _returnvalue_4 (Class|TempestGeneralLibrary|GetSpecialPropertyOfTag (Class|TempestPropertiesComponent|GetSpecialProperties _returnvalue_3) "(TagName=\"Property.Special.Behavior.Execution\")"))
      (bind _asbp_enemy_execution_behavior (Utilities|Casting|CastToBP_EnemyExecutionBehavior _returnvalue_4))
      (for _array_element (Variables|/TempestCombatFramework/BehaviorProperties/BP_EnemyExecutionBehavior.BP_EnemyExecutionBehavior_C|GetExecution%20Properties _asbp_enemy_execution_behavior)
        (if (Utilities|IsValidClass (.ConditionToUse (Utilities|Struct|BreakS_AssasinationProperties _array_element)))
          (bind _returnvalue_5 (Class|TempestGeneralLibrary|GetObjectOfClass (Variables|Default|GetConditions%20Created) (.ConditionToUse (Utilities|Struct|BreakS_AssasinationProperties _array_element))))
          (Utilities|IsValid _returnvalue_5
            (:Is%20Valid
              (bind _asbp_owner_target_condition (Utilities|Casting|CastToBP_OwnerTargetCondition _returnvalue_5))
              (Default|UpdateOwnerActor&Target _asbp_owner_target_condition (Variables|Default|GetOwner%20Character) _foundcombattarget_2)
              (bind _returnvalue_6 (Class|TempestBaseConditionObject|GetConditionResult _asbp_owner_target_condition))
              (if _returnvalue_6
                (return _array_element)))
            (:Is%20Not%20Valid
              (bind _returnvalue_7 (Game|ConstructObjectfromClass _owner_character (.ConditionToUse (Utilities|Struct|BreakS_AssasinationProperties _array_element)) _owner_character _foundcombattarget_2))
              (Utilities|Array|Add (Variables|Default|GetConditions%20Created) _returnvalue_7)
              (Default|UpdateOwnerActor&Target _returnvalue_7 (Variables|Default|GetOwner%20Character) _foundcombattarget_2)
              (bind _returnvalue_8 (Class|TempestBaseConditionObject|GetConditionResult _returnvalue_7))
              (if _returnvalue_8
                (return _array_element))))
          (else
            (return _array_element))))
      (return ""))))