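; BP_GS_CharcterNormalDeathAbility is a gameplay ability that plays a character's death animation.
; It can be performed only when the performing actor's Health attribute, read from its Tempest attributes component, is at or below its minimum value.
; On start it plays DeathMontage if valid, otherwise a random montage from the ability montages tagged List.One.
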(event EventStartAbility
  (bind _death_montage (Variables|Default|GetDeath%20Montage))
  (|CallParentFunction)
  (Utilities|IsValid _death_montage
    (:Is%20Valid
      (CallFunction|PlayAbilityMontage _death_montage 1.0 "Duration" 0.0 "None" true))
    (:Is%20Not%20Valid
      (bind _list_of_montages (CallFunction|GetAbilityMontagesOfTag "(TagName=\"List.One\")"))
      (CallFunction|PlayAbilityMontage (.OutItem (Utilities|Array|Random _list_of_montages)) 1.0 "Duration" 0.0 "None" true))))

(event EventEndAbility
  (|CallParentFunction))

(fn CanPerformAbility
  (bind _currentperformingactor (Class|TempestBaseAbilityObject|GetPerformingActor))
  (bind _returnvalue (Actor|GetComponentbyClass _currentperformingactor "/Script/TempestCombatFramework.TempestAttributesComponents"))
  (bind _returnvalue_2 (Class|TempestAttributesComponents|GetAttributeOfGameplayTag _returnvalue "(TagName=\"Attribute.Health\")"))
  (bind _attributevalues (Variables|/Script/TempestCombatFramework.TempestBaseAttributeObject|GetAttributeValues _returnvalue_2))
  (bind (_attributevalue _minattributevalue) (Utilities|Struct|BreakAttributeProperties _attributevalues))
  (return (<= _attributevalue _minattributevalue)))