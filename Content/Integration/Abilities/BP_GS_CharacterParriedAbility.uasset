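; Tempest combat ability that puts a character into a parried reaction when its posture breaks.
; Activation requires being alive, not invincible, not already running the ability, and incoming posture damage reaching the attribute's minimum.
; That damage comes from the received attack's impact property, using Block values in blocking states and Hit otherwise.
; On start, it drains posture with a huge negative modifier and plays a random parried montage.
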(event EventStartAbility
  (|CallParentFunction)
  (Class|TempestBaseAttributeObject|ModifyAttribute (Class|TempestAttributesComponents|GetAttributeOfGameplayTag (Actor|GetComponentbyClass (Class|TempestBaseAbilityObject|GetPerformingActor) "/Script/TempestCombatFramework.TempestAttributesComponents") "(TagName=\"Attribute.Posture\")") -5e+06)
  (bind _list_of_montages (CallFunction|GetAbilityMontagesOfTag "(TagName=\"List.One\")"))
  (Variables|Default|SetParried%20Montages _list_of_montages)
  (CallFunction|PlayAbilityMontage (.OutItem (Utilities|Array|Random (Variables|Default|GetParried%20Montages))) 1.0 "MontageLength" 0.0 "None" true))

(fn CanPerformAbility
  (bind _currentperformingactor (Class|TempestBaseAbilityObject|GetPerformingActor))
  (bind _currentperformingactor_2 (Class|TempestBaseAbilityObject|GetPerformingActor))
  (bind _returnvalue (Actor|GetComponentbyClass _currentperformingactor "/Script/TempestCombatFramework.TempestBaseStateManagerComponent"))
  (bind _returnvalue_2 (Actor|GetComponentbyClass _currentperformingactor_2 "/Script/TempestCombatFramework.TempestAttributesComponents"))
  (bind _returnvalue_3 (Class|TempestBaseStateManagerComponent|GetCurrentActiveState _returnvalue))
  (bind _returnvalue_4 (Class|TempestAttributesComponents|GetAttributeOfGameplayTag _returnvalue_2 "(TagName=\"Attribute.Posture\")"))
  (bind _stategameplaytag (Variables|/Script/TempestCombatFramework.TempestBaseStateObject|GetStateGameplayTag _returnvalue_3))
  (bind _attributevalues (Variables|/Script/TempestCombatFramework.TempestBaseAttributeObject|GetAttributeValues _returnvalue_4))
  (bind (_attributevalue _minattributevalue) (Utilities|Struct|BreakAttributeProperties _attributevalues))
  (if (and (!= (Variables|/Script/TempestCombatFramework.TempestBaseStateObject|GetStateGameplayTag (Class|TempestBaseStateManagerComponent|GetCurrentActiveState (Actor|GetComponentbyClass (Variables|Default|GetOwner%20Character) "/Script/TempestCombatFramework.TempestBaseStateManagerComponent"))) "(TagName=\"State.Death\")") (not (GameplayTags|HasTag (Class|TempestCombatComponent|GetCombatStatus (Actor|GetComponentbyClass (Class|TempestBaseAbilityObject|GetPerformingActor) "/Script/TempestCombatFramework.TempestCombatComponent")) "(TagName=\"Status.Combat.Invincible\")")))
    (Utilities|IsValid _returnvalue_4
      (:Is%20Valid
        (bind _asbp_damage_per_impact_property (Utilities|Casting|CastToBP_DamagePerImpactProperty (Utilities|Struct|BreakInstancedImpactProperties (Class|TempestAttackPropertiesObject|GetImpactPropertyOfGameplayTag (Variables|/Script/TempestCombatFramework.TempestCombatComponent|GetReceivedAttackProperty (Actor|GetComponentbyClass (Class|TempestBaseAbilityObject|GetPerformingActor) "/TempestCombatFramework/Components/BP_TempestBaseCombatComponent.BP_TempestBaseCombatComponent_C")) "(TagName=\"Property.Impact.Damage Per Result\")"))))
        (bind _return_value (Default|FindDamagetoApplyOfGameplayTag _asbp_damage_per_impact_property "(TagName=\"Attribute.Posture\")" (select (or (== _stategameplaytag "(TagName=\"State.Trying To Block\")") (== _stategameplaytag "(TagName=\"State.Normal Block\")")) "(TagName=\"Impact.Result.Block\")" "(TagName=\"Impact.Result.Hit\")")))
        (bind _output_get (Variables|Default|SetValue%20To%20Set%20Posture%20To _return_value))
        (return (and (<= (- _attributevalue _output_get) _minattributevalue) (not (CallFunction|GetIsCurrentAbilityActive)))))
      (:Is%20Not%20Valid
        (return false)))
    (else
      (return false))))