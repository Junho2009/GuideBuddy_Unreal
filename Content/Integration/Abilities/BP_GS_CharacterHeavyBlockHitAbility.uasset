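; Ability that plays a character's reaction to blocking a heavy, leap-type attack.
; It can run only while alive, blocking or trying to block, with the combat target within a frontal yaw arc and the received attack tagged as Leap.
; On start it plays a random tagged blocked montage and applies the equipped weapon's block impact effect through the owner's defense property.
; Cancelling ends the ability.
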(event EventStartAbility
  (bind _currentperformingactor (Class|TempestBaseAbilityObject|GetPerformingActor))
  (bind _returnvalue (Actor|GetComponentbyClass _currentperformingactor "/TempestCombatFramework/Components/BP_TempestBaseCombatComponent.BP_TempestBaseCombatComponent_C"))
  (|CallParentFunction)
  (bind _list_of_montages (CallFunction|GetAbilityMontagesOfTag "(TagName=\"List.One\")"))
  (Variables|Default|SetBlocked%20Montages _list_of_montages)
  (CallFunction|PlayAbilityMontage (.OutItem (Utilities|Array|Random (Variables|Default|GetBlocked%20Montages))) 1.0 "MontageLength" 0.0 "None" true)
  (bind _found_impact_effect (Default|GetImpactEffectClassOfTag (Variables|/TempestCombatFramework/Actors/Weapons/BP_BaseWeapon.BP_BaseWeapon_C|GetData%20Asset%20Info%20Reference (Default|GetEquippedWeapon _returnvalue)) "(TagName=\"Impact.Effect.Block\")"))
  (Class|TempestDefensePropertiesObject|ApplyHitEffectOfClass (Variables|/Script/TempestCombatFramework.TempestCombatComponent|GetOwnerDefenseProperty _returnvalue) _found_impact_effect))

(event EventCancelAbility
  (|CallParentFunction)
  (Class|TempestBaseAbilityObject|EndAbility))

(fn CanPerformAbility
  (bind _currentperformingactor (Class|TempestBaseAbilityObject|GetPerformingActor))
  (bind _currentperformingactor_2 (Class|TempestBaseAbilityObject|GetPerformingActor))
  (bind _returnvalue (Actor|GetComponentbyClass _currentperformingactor_2 "/Script/TempestCombatFramework.TempestBaseStateManagerComponent"))
  (bind _returnvalue_2 (Class|TempestBaseStateManagerComponent|GetCurrentActiveState _returnvalue))
  (bind _stategameplaytag (Variables|/Script/TempestCombatFramework.TempestBaseStateObject|GetStateGameplayTag _returnvalue_2))
  (if (and (!= _stategameplaytag "(TagName=\"State.Death\")") (or (== _stategameplaytag "(TagName=\"State.Trying To Block\")") (== _stategameplaytag "(TagName=\"State.Normal Block\")")))
    (bind _returnvalue_3 (Class|TempestMathLibrary|GetAnglesBetweenActors _currentperformingactor (Class|TempestCombatComponent|GetCombatTarget (Actor|GetComponentbyClass _currentperformingactor "/Script/TempestCombatFramework.TempestCombatComponent"))))
    (return (and (Math|Float|InRange(Float) (.yaw _returnvalue_3) -65.0 65.0) (== (Variables|/Script/TempestCombatFramework.TempestAttackPropertiesObject|GetAttackPropertyTag (Variables|/Script/TempestCombatFramework.TempestCombatComponent|GetReceivedAttackProperty (Actor|GetComponentbyClass (Class|TempestBaseAbilityObject|GetPerformingActor) "/TempestCombatFramework/Components/BP_TempestBaseCombatComponent.BP_TempestBaseCombatComponent_C"))) "(TagName=\"Property.Attack.Leap\")")))
    (else
      (return false))))