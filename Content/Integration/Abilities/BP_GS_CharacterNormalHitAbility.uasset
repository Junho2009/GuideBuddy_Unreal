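; Tempest combat ability that plays a character's reaction to normal, thrust, gunshot or normal-knock hits, unless invincible or on cooldown.
; It picks a front or back montage from the yaw toward the attacker, defaulting to front if the attack property cast fails; two other montage branches are unwired.
; The equipped weapon's default impact effect is applied through the defense property.
; Ending or cancelling returns player-controlled characters to Idle state.
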(event EventStartAbility
  (bind _currentperformingactor (Class|TempestBaseAbilityObject|GetPerformingActor))
  (bind _currentperformingactor_2 (Class|TempestBaseAbilityObject|GetPerformingActor))
  (bind _returnvalue (Actor|GetComponentbyClass _currentperformingactor "/TempestCombatFramework/Components/BP_TempestBaseCombatComponent.BP_TempestBaseCombatComponent_C"))
  (|CallParentFunction)
  (bind _list_of_montages (CallFunction|GetAbilityMontagesOfTag "(TagName=\"List.One\")"))
  (Variables|Default|SetHit%20Reaction%20Montages _list_of_montages)
  (bind _asbp_normal_attack_property (Utilities|Casting|CastToBP_NormalAttackProperty (Variables|/Script/TempestCombatFramework.TempestCombatComponent|GetReceivedAttackProperty (Actor|GetComponentbyClass (Class|TempestBaseAbilityObject|GetPerformingActor) "/Script/TempestCombatFramework.TempestCombatComponent")))
    (:then
      (Variables|Default|SetNormal%20Attack%20Property _asbp_normal_attack_property)
      (bind _returnvalue_2 (Class|TempestMathLibrary|GetAnglesBetweenActors _currentperformingactor_2 (Class|TempestAttackPropertiesObject|GetAttackPropertyOwner (Variables|/Script/TempestCombatFramework.TempestCombatComponent|GetReceivedAttackProperty (Actor|GetComponentbyClass _currentperformingactor_2 "/Script/TempestCombatFramework.TempestCombatComponent")))))
      (Variables|Default|SetDirection (select (Math|Float|InRange(Float) (.yaw _returnvalue_2) -9e+01 9e+01) "NewEnumerator8" "NewEnumerator9"))
      (switch Utilities|FlowControl|Switch|SwitchonE_4DDirection (Variables|Default|GetDirection)
        (:NewEnumerator8
          (CallFunction|PlayAbilityMontage (Utilities|Array|Get(acopy) (Variables|Default|GetHit%20Reaction%20Montages)) 1.0 "MontageLength" 0.0 "None" true :!label _label))
        (:NewEnumerator9
          (CallFunction|PlayAbilityMontage (Utilities|Array|Get(acopy) (Variables|Default|GetHit%20Reaction%20Montages) 3) 1.0 "MontageLength" 0.0 "None" true))))
    (:CastFailed
      (goto _label)))
  (bind _found_impact_effect (Default|GetImpactEffectClassOfTag (Variables|/TempestCombatFramework/Actors/Weapons/BP_BaseWeapon.BP_BaseWeapon_C|GetData%20Asset%20Info%20Reference (Default|GetEquippedWeapon _returnvalue)) "(TagName=\"Impact.Effect.Default\")"))
  (Class|TempestDefensePropertiesObject|ApplyHitEffectOfClass (Variables|/Script/TempestCombatFramework.TempestCombatComponent|GetOwnerDefenseProperty _returnvalue) _found_impact_effect))

(event EventEndAbility
  (bind _owner_character (Variables|Default|GetOwner%20Character))
  (bind _returnvalue (Actor|GetComponentbyClass _owner_character "/Script/TempestCombatFramework.TempestBaseStateManagerComponent"))
  (|CallParentFunction)
  (if (Pawn|IsPlayerControlled _owner_character)
    (Class|TempestBaseStateManagerComponent|PerformStateOfClass _returnvalue (Utilities|GetClass (Class|TempestBaseStateManagerComponent|GetStateOfGameplayTag _returnvalue "(TagName=\"State.Idle\")")))))

(event EventCancelAbility
  (|CallParentFunction)
  (Class|TempestBaseAbilityObject|EndAbility))

(fn CanPerformAbility
  (bind _currentperformingactor (Class|TempestBaseAbilityObject|GetPerformingActor))
  (bind _returnvalue (Actor|GetComponentbyClass _currentperformingactor "/TempestCombatFramework/Components/BP_TempestBaseCombatComponent.BP_TempestBaseCombatComponent_C"))
  (bind _receivedattackproperty (Variables|/Script/TempestCombatFramework.TempestCombatComponent|GetReceivedAttackProperty _returnvalue))
  (bind _attackpropertytag (Variables|/Script/TempestCombatFramework.TempestAttackPropertiesObject|GetAttackPropertyTag _receivedattackproperty))
  (if (not (GameplayTags|HasTag (Class|TempestCombatComponent|GetCombatStatus _returnvalue) "(TagName=\"Status.Combat.Invincible\")"))
    (return (and (Math|Boolean|ORBoolean (== _attackpropertytag "(TagName=\"Property.Attack.Normal\")") (== _attackpropertytag "(TagName=\"Property.Attack.Thrust\")") (== _attackpropertytag "(TagName=\"Property.Attack.Projectile.GunShot\")") (== _attackpropertytag "(TagName=\"Property.Attack.Normal & Knock\")")) (not (Class|TempestBaseAbilityObject|GetIsAbilityonCooldown))))
    (else
      (return false))))