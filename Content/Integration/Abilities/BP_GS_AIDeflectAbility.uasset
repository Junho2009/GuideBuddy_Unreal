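; AI ability that deflects an incoming attack while blocking in combat with an equipped weapon.
; It requires a non-leap attack from an attacker within a frontal yaw cone, and a blocked-hit count reaching DeflectCount.
; On start it resets that count, picks a montage by swing direction (random for non-normal attacks), and notifies the attacker's active ability.
; It then applies the weapon's deflect impact effect and re-rolls DeflectCount, varying deflect timing.
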(event EventStartAbility
  (bind _currentperformingactor (Class|TempestBaseAbilityObject|GetPerformingActor))
  (bind _returnvalue (Actor|GetComponentbyClass _currentperformingactor "/TempestCombatFramework/Components/BP_TempestBaseCombatComponent.BP_TempestBaseCombatComponent_C"))
  (|CallParentFunction)
  (Class|TempestBaseStatisticObject|ResetStatisticValue (Class|TempestStatisticsComponent|GetStatisticOfGameplayTag (Actor|GetComponentbyClass (Class|TempestBaseAbilityObject|GetPerformingActor) "/TempestCombatFramework/Components/BP_TempestStatisticsComponent.BP_TempestStatisticsComponent_C") "(TagName=\"Statistic.Count.Block Hit\")"))
  (bind _list_of_montages (CallFunction|GetAbilityMontagesOfTag "(TagName=\"List.One\")"))
  (Variables|Default|SetMontages _list_of_montages)
  (bind _asbp_normal_attack_property (Utilities|Casting|CastToBP_NormalAttackProperty (Variables|/Script/TempestCombatFramework.TempestCombatComponent|GetReceivedAttackProperty (Actor|GetComponentbyClass (Class|TempestBaseAbilityObject|GetPerformingActor) "/Script/TempestCombatFramework.TempestCombatComponent")))
    (:then
      (switch Utilities|FlowControl|Switch|SwitchonE_SwingDirection (Variables|/TempestCombatFramework/AttackProperties/BP_NormalAttackProperty.BP_NormalAttackProperty_C|GetSwing%20Direction _asbp_normal_attack_property)
        (:NewEnumerator3
          (CallFunction|PlayAbilityMontage (Utilities|Array|Get(acopy) (Variables|Default|GetMontages)) 1.0 "MontageLength" 0.0 "None" true :!label _label))
        (:NewEnumerator5
          (goto _label))
        (:NewEnumerator8
          (goto _label))
        (:NewEnumerator9
          (CallFunction|PlayAbilityMontage (Utilities|Array|Get(acopy) (Variables|Default|GetMontages) 1) 1.0 "MontageLength" 0.0 "None" true :!label _label_2))
        (:NewEnumerator10
          (goto _label))
        (:NewEnumerator11
          (goto _label))
        (:NewEnumerator12
          (goto _label_2))
        (:NewEnumerator13
          (goto _label_2))))
    (:CastFailed
      (CallFunction|PlayAbilityMontage (.OutItem (Utilities|Array|Random (Variables|Default|GetMontages))) 1.0 "Duration" 0.0 "None" true)))
  (Class|BPITempestAbilitiesandStates|InformTargetOfDeflect(Message) (Class|TempestBaseAbilityManagerComponent|GetCurrentActiveAbility (Actor|GetComponentbyClass (Class|TempestAttackPropertiesObject|GetAttackPropertyOwner (Variables|/Script/TempestCombatFramework.TempestCombatComponent|GetReceivedAttackProperty (Actor|GetComponentbyClass (Class|TempestBaseAbilityObject|GetPerformingActor) "/TempestCombatFramework/Components/BP_TempestBaseCombatComponent.BP_TempestBaseCombatComponent_C"))) "/Script/TempestCombatFramework.TempestBaseAbilityManagerComponent")))
  (bind _found_impact_effect (Default|GetImpactEffectClassOfTag (Variables|/TempestCombatFramework/Actors/Weapons/BP_BaseWeapon.BP_BaseWeapon_C|GetData%20Asset%20Info%20Reference (Default|GetEquippedWeapon _returnvalue)) "(TagName=\"Impact.Effect.Deflect\")"))
  (Class|TempestDefensePropertiesObject|ApplyHitEffectOfClass (Variables|/Script/TempestCombatFramework.TempestCombatComponent|GetOwnerDefenseProperty _returnvalue) _found_impact_effect)
  (Variables|Default|SetDeflect%20Count (Math|Conversions|ToFloat(Integer) (Math|Random|RandomIntegerinRange 0 2))))

(event EventCancelAbility
  (|CallParentFunction)
  (Class|TempestBaseAbilityObject|EndAbility))

(fn CanPerformAbility
  (bind _currentperformingactor (Class|TempestBaseAbilityObject|GetPerformingActor))
  (bind _returnvalue (Actor|GetComponentbyClass _currentperformingactor "/TempestCombatFramework/Components/BP_TempestBaseCombatComponent.BP_TempestBaseCombatComponent_C"))
  (bind _returnvalue_2 (Actor|GetComponentbyClass _currentperformingactor "/Script/TempestCombatFramework.TempestBaseStateManagerComponent"))
  (bind _returnvalue_3 (Class|TempestBaseStateManagerComponent|GetCurrentActiveState _returnvalue_2))
  (bind _receivedattackproperty (Variables|/Script/TempestCombatFramework.TempestCombatComponent|GetReceivedAttackProperty _returnvalue))
  (bind _stategameplaytag (Variables|/Script/TempestCombatFramework.TempestBaseStateObject|GetStateGameplayTag _returnvalue_3))
  (Utilities|IsValid (Class|TempestBaseStateManagerComponent|GetCurrentActiveState _returnvalue_2)
    (:Is%20Valid
      (bind _returnvalue_4 (Class|TempestMathLibrary|GetAnglesBetweenActors (Class|TempestBaseAbilityObject|GetPerformingActor) (Class|TempestAttackPropertiesObject|GetAttackPropertyOwner _receivedattackproperty)))
      (return (Math|Boolean|ANDBoolean (GameplayTags|HasTag (Class|TempestCombatComponent|GetCombatStatus _returnvalue) "(TagName=\"Status.Combat.InCombat\")") (Utilities|IsValid (Default|GetEquippedWeapon _returnvalue)) (Math|Float|InRange(Float) (.yaw _returnvalue_4) -65.0 65.0) (or (== _stategameplaytag "(TagName=\"State.Normal Block\")") (== _stategameplaytag "(TagName=\"State.Trying To Block\")")) (>= (Variables|/Script/TempestCombatFramework.TempestBaseStatisticObject|GetStatisticCurrentValue (Class|TempestStatisticsComponent|GetStatisticOfGameplayTag (Actor|GetComponentbyClass (Class|TempestBaseAbilityObject|GetPerformingActor) "/Script/TempestCombatFramework.TempestStatisticsComponent") "(TagName=\"Statistic.Count.Block Hit\")")) (Variables|Default|GetDeflect%20Count)) (!= (Variables|/Script/TempestCombatFramework.TempestAttackPropertiesObject|GetAttackPropertyTag _receivedattackproperty) "(TagName=\"Property.Attack.Leap\")"))))
    (:Is%20Not%20Valid
      (return false))))