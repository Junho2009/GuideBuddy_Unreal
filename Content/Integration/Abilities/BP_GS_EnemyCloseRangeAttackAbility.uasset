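; Enemy close-range attack ability for the Tempest combat components, playing montages tagged List.One and setting the performer to the Attack state.
; It is performable only when montages exist and the combat target is within short range and neither dead nor parried.
; Each start advances a wrapping montage index, which resets when the ability ends, cancels or another ability activates.
; Deflect and clash notifications attempt the performer's Deflected or Clashed state.
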(event Custom|OnAbilityActivation_Event
  (params (ActivatedAbility :type Tempest%20Base%20Ability%20Object%20Object%20Reference))
  (if (!= ActivatedAbility self)
    (Variables|Default|SetChoosen%20Attack%20Index 0)))

(event EventStartAbility
  (bind _currentperformingactor (Class|TempestBaseAbilityObject|GetPerformingActor))
  (bind _attack_montages (Variables|AttackMontagesToPickFrom|GetAttack%20Montages))
  (bind _returnvalue (Actor|GetComponentbyClass _currentperformingactor "/Script/TempestCombatFramework.TempestBaseStateManagerComponent"))
  (|CallParentFunction)
  (CallFunction|PlayAbilityMontage (Utilities|Array|Get(acopy) _attack_montages (Variables|Default|GetChoosen%20Attack%20Index)) 1.0 "Duration" 0.0 "None" true)
  (if (> (+ (Variables|Default|GetChoosen%20Attack%20Index) 1) (Utilities|Array|LastIndex _attack_montages))
    (Variables|Default|SetChoosen%20Attack%20Index 0)
    (else
      (Variables|Default|SetChoosen%20Attack%20Index (+ (Variables|Default|GetChoosen%20Attack%20Index) 1))))
  (Class|TempestBaseStateManagerComponent|SetCurrentActiveState _returnvalue (Class|TempestBaseStateManagerComponent|GetStateOfGameplayTag _returnvalue "(TagName=\"State.Attack\")")))

(event EventInformTargetOfDeflect
  (bind _currentperformingactor (Class|TempestBaseAbilityObject|GetPerformingActor))
  (bind _returnvalue (Actor|GetComponentbyClass _currentperformingactor "/Script/TempestCombatFramework.TempestBaseStateManagerComponent"))
  (Class|TempestBaseStateManagerComponent|TryPerformStateOfClass _returnvalue (Utilities|GetClass (Class|TempestBaseStateManagerComponent|GetStateOfGameplayTag _returnvalue "(TagName=\"State.Deflected\")")) true))

(event EventCancelAbility
  (|CallParentFunction)
  (Class|TempestBaseAbilityObject|EndAbility))

(event EventConstructAbility
  (|CallParentFunction)
  (bind _list_of_montages (CallFunction|GetAbilityMontagesOfTag "(TagName=\"List.One\")"))
  (Variables|AttackMontagesToPickFrom|SetAttack%20Montages _list_of_montages)
  (EventDispatchers|AssignOnAbilityActivation (Actor|GetComponentbyClass (Class|TempestBaseAbilityObject|GetPerformingActor) "/Script/TempestCombatFramework.TempestBaseAbilityManagerComponent") (EventDispatchers|CreateEvent :!event Custom|OnAbilityActivation_Event)))

(event EventInformTargetOfClash
  (bind _currentperformingactor (Class|TempestBaseAbilityObject|GetPerformingActor))
  (bind _returnvalue (Actor|GetComponentbyClass _currentperformingactor "/Script/TempestCombatFramework.TempestBaseStateManagerComponent"))
  (Class|TempestBaseStateManagerComponent|TryPerformStateOfClass _returnvalue (Utilities|GetClass (Class|TempestBaseStateManagerComponent|GetStateOfGameplayTag _returnvalue "(TagName=\"State.Clashed\")")) true))

(event EventEndAbility
  (Variables|Default|SetChoosen%20Attack%20Index 0)
  (|CallParentFunction))

(fn CanPerformAbility
  (bind _currentperformingactor (Class|TempestBaseAbilityObject|GetPerformingActor))
  (bind _currentperformingactor_2 (Class|TempestBaseAbilityObject|GetPerformingActor))
  (bind _returnvalue (Actor|GetComponentbyClass _currentperformingactor "/Script/TempestCombatFramework.TempestCombatComponent"))
  (bind _foundcombattarget (Class|TempestCombatComponent|GetCombatTarget _returnvalue))
  (bind _returnvalue_2 (Actor|GetComponentbyClass _foundcombattarget "/Script/TempestCombatFramework.TempestBaseStateManagerComponent"))
  (bind _returnvalue_3 (Class|TempestBaseStateManagerComponent|GetCurrentActiveState _returnvalue_2))
  (bind _stategameplaytag (Variables|/Script/TempestCombatFramework.TempestBaseStateObject|GetStateGameplayTag _returnvalue_3))
  (bind _list_of_montages (CallFunction|GetAbilityMontagesOfTag "(TagName=\"List.One\")"))
  (if (or (Utilities|Array|IsValidIndex (Variables|AttackMontagesToPickFrom|GetAttack%20Montages)) (> (Utilities|Array|Length _list_of_montages) 0))
    (bind _returnvalue_4 (Class|TempestMathLibrary|GetDistanceBetweenActors _currentperformingactor_2 (Class|TempestCombatComponent|GetCombatTarget (Actor|GetComponentbyClass _currentperformingactor_2 "/Script/TempestCombatFramework.TempestCombatComponent"))))
    (return (and (Math|Float|InRange(Float) _returnvalue_4 1.0 3e+02) (and (!= _stategameplaytag "(TagName=\"State.Death\")") (!= _stategameplaytag "(TagName=\"State.Parried\")"))))
    (else
      (return false))))

(fn GetAbilityProjectile
  (return 0))

(fn GetAssociatedPassiveAbilities
  (return 0))

(fn GetBlockTimeSinceLastClicked
  (return 0.0))

(fn GetMontageCounterforAbility
  (return 0))

(fn GetMontageOfGameplayTag
  (params (Montage%20Tag :type Gameplay%20Tag%20Structure))
  (return 0))

(fn GetStrafingValues
  (return 0.0 "0, 0, 0"))

(fn ProcessIncomingAttack
  (params (Incoming%20Attack%20Type :type Gameplay%20Tag%20Structure))
  (return false))