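; Player deflect (parry) ability, allowed in combat with a weapon when block was just pressed and the attacker is roughly in front, excluding leap attacks.
; It picks a montage by incoming swing direction, notifies the attacker's active ability and applies the weapon's deflect impact effect.
; On end, it resumes the block loop if right mouse is held and block is available, otherwise returns to idle.
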(event EventStartAbility
  (bind _currentperformingactor (Class|TempestBaseAbilityObject|GetPerformingActor))
  (bind _returnvalue (Actor|GetComponentbyClass _currentperformingactor "/TempestCombatFramework/Components/BP_TempestBaseCombatComponent.BP_TempestBaseCombatComponent_C"))
  (|CallParentFunction)
  (bind _list_of_montages (CallFunction|GetAbilityMontagesOfTag "(TagName=\"List.One\")"))
  (Variables|Default|SetMontages _list_of_montages)
  (bind _asbp_normal_attack_property (Utilities|Casting|CastToBP_NormalAttackProperty (Variables|/Script/TempestCombatFramework.TempestCombatComponent|GetReceivedAttackProperty (Actor|GetComponentbyClass (Class|TempestBaseAbilityObject|GetPerformingActor) "/Script/TempestCombatFramework.TempestCombatComponent")))
    (:then
      (switch Utilities|FlowControl|Switch|SwitchonE_SwingDirection (Variables|/TempestCombatFramework/AttackProperties/BP_NormalAttackProperty.BP_NormalAttackProperty_C|GetSwing%20Direction _asbp_normal_attack_property)
        (:NewEnumerator3
          (CallFunction|PlayAbilityMontage (Utilities|Array|Get(acopy) (Variables|Default|GetMontages)) 1.0 "MontageLength" 0.0 "None" true :!label _label))
        (:NewEnumerator5
          (goto _label))
        (:NewEnumerator8
          (goto _label))
        (:NewEnumerator9
          (CallFunction|PlayAbilityMontage (Utilities|Array|Get(acopy) (Variables|Default|GetMontages) 1) 1.0 "MontageLength" 0.0 "None" true :!label _label_2))
        (:NewEnumerator10
          (goto _label))
        (:NewEnumerator11
          (goto _label))
        (:NewEnumerator12
          (goto _label_2))
        (:NewEnumerator13
          (goto _label_2))))
    (:CastFailed
      (CallFunction|PlayAbilityMontage (.OutItem (Utilities|Array|Random (Variables|Default|GetMontages))) 1.0 "Duration" 0.0 "None" true)))
  (Class|BPITempestAbilitiesandStates|InformTargetOfDeflect(Message) (Class|TempestBaseAbilityManagerComponent|GetCurrentActiveAbility (Actor|GetComponentbyClass (Class|TempestAttackPropertiesObject|GetAttackPropertyOwner (Variables|/Script/TempestCombatFramework.TempestCombatComponent|GetReceivedAttackProperty (Actor|GetComponentbyClass (Class|TempestBaseAbilityObject|GetPerformingActor) "/TempestCombatFramework/Components/BP_TempestBaseCombatComponent.BP_TempestBaseCombatComponent_C"))) "/Script/TempestCombatFramework.TempestBaseAbilityManagerComponent")))
  (bind _found_impact_effect (Default|GetImpactEffectClassOfTag (Variables|/TempestCombatFramework/Actors/Weapons/BP_BaseWeapon.BP_BaseWeapon_C|GetData%20Asset%20Info%20Reference (Default|GetEquippedWeapon _returnvalue)) "(TagName=\"Impact.Effect.Deflect\")"))
  (Class|TempestDefensePropertiesObject|ApplyHitEffectOfClass (Variables|/Script/TempestCombatFramework.TempestCombatComponent|GetOwnerDefenseProperty _returnvalue) _found_impact_effect))

(event EventEndAbility
  (bind _tempestabilitycomponent (CallFunction|GetTempestAbilityComponent))
  (bind _owner_character (Variables|Default|GetOwner%20Character))
  (bind _returnvalue (Actor|GetComponentbyClass _owner_character "/Script/TempestCombatFramework.TempestBaseStateManagerComponent"))
  (bind _returnvalue_2 (Class|TempestBaseAbilityManagerComponent|GetAbilityOfGameplayTag _tempestabilitycomponent "(TagName=\"Ability.Block.Loop\")"))
  (bind _returnvalue_3 (Utilities|GetClass _returnvalue_2))
  (|CallParentFunction)
  (if (Utilities|Enum|Equal(Enum) (Class|TempestBaseInputComponent|GetInputActionCurrentTriggerEvent (Actor|GetComponentbyClass (Class|TempestBaseAbilityObject|GetPerformingActor) "/Script/TempestCombatFramework.TempestBaseInputComponent") "/TempestCombatFramework/Input/RightMouse_Input.RightMouse_Input") "Triggered")
    (if (Class|TempestBaseAbilityManagerComponent|GetCanPerformAbilityOfClass _tempestabilitycomponent _returnvalue_3)
      (Class|TempestBaseAbilityManagerComponent|PerformAbilityOfClass (CallFunction|GetTempestAbilityComponent) _returnvalue_3)
      (Class|TempestBaseStateManagerComponent|SetCurrentActiveState _returnvalue (Class|TempestBaseStateManagerComponent|GetStateOfGameplayTag _returnvalue "(TagName=\"State.Normal Block\")"))
      (else
        (Class|BPITCFGeneralInterface|AssignMoveset(Message) (Components|SkeletalMesh|GetAnimInstance (Variables|/Script/Engine.Character|GetMesh _owner_character)) "NewEnumerator1" :!label _label)
        (Class|TempestBaseStateManagerComponent|PerformStateOfClass _returnvalue (Utilities|GetClass (Class|TempestBaseStateManagerComponent|GetStateOfGameplayTag _returnvalue "(TagName=\"State.Idle\")")))))
    (else
      (goto _label))))

(event EventCancelAbility
  (|CallParentFunction)
  (Class|TempestBaseAbilityObject|EndAbility))

(fn CanPerformAbility
  (bind _owner_character (Variables|Default|GetOwner%20Character))
  (bind _owner_character_2 (Variables|Default|GetOwner%20Character))
  (bind _returnvalue (Actor|GetComponentbyClass _owner_character_2 "/TempestCombatFramework/Components/BP_TempestBaseCombatComponent.BP_TempestBaseCombatComponent_C"))
  (bind _returnvalue_2 (Actor|GetComponentbyClass _owner_character "/Script/TempestCombatFramework.TempestBaseStateManagerComponent"))
  (bind _receivedattackproperty (Variables|/Script/TempestCombatFramework.TempestCombatComponent|GetReceivedAttackProperty _returnvalue))
  (Utilities|IsValid (Class|TempestBaseStateManagerComponent|GetCurrentActiveState _returnvalue_2)
    (:Is%20Valid
      (bind _returnvalue_3 (Class|TempestMathLibrary|GetAnglesBetweenActors (Variables|Default|GetOwner%20Character) (Class|TempestAttackPropertiesObject|GetAttackPropertyOwner _receivedattackproperty)))
      (bind _key_time_down (CallFunction|CalculateTimeDown))
      (return (Math|Boolean|ANDBoolean (GameplayTags|HasTag (Class|TempestCombatComponent|GetCombatStatus _returnvalue) "(TagName=\"Status.Combat.InCombat\")") (Utilities|IsValid (Default|GetEquippedWeapon _returnvalue)) (Math|Float|InRange(Float) (.yaw _returnvalue_3) -65.0 65.0) (or (== (Variables|/Script/TempestCombatFramework.TempestBaseStateObject|GetStateGameplayTag (Class|TempestBaseStateManagerComponent|GetCurrentActiveState _returnvalue_2)) "(TagName=\"State.Normal Block\")") (and (CallFunction|GetIsCurrentAbilityActive) (Utilities|Enum|Equal(Enum) (Class|TempestBaseInputComponent|GetInputActionCurrentTriggerEvent (Actor|GetComponentbyClass (Class|TempestBaseAbilityObject|GetPerformingActor) "/Script/TempestCombatFramework.TempestBaseInputComponent") "/TempestCombatFramework/Input/RightMouse_Input.RightMouse_Input") "Triggered"))) (<= _key_time_down 0.18) (!= (Variables|/Script/TempestCombatFramework.TempestAttackPropertiesObject|GetAttackPropertyTag _receivedattackproperty) "(TagName=\"Property.Attack.Leap\")"))))
    (:Is%20Not%20Valid
      (return false))))

(fn CalculateTimeDown
  (bind _asplayer_controller (Utilities|Casting|CastToPlayerController (Variables|Default|GetOwner%20Controller)))
  (for _array_element (CallFunction|GetKeysOfInputAction "/Game/Integration/GS_Player_InputMappings.GS_Player_InputMappings" "/TempestCombatFramework/Input/RightMouse_Input.RightMouse_Input")
    (if (and (> (Class|PlayerController|GetInputKeyTimeDown _asplayer_controller _array_element) 0.0) (> (Class|PlayerController|GetInputKeyTimeDown _asplayer_controller _array_element) (LocalVariables|GetLocal%20Key%20Time%20Down)))
      (LocalVariables|SetLocal%20Key%20Time%20Down (Class|PlayerController|GetInputKeyTimeDown _asplayer_controller _array_element))))
  (return (select (> (LocalVariables|GetLocal%20Key%20Time%20Down) 0.0) (LocalVariables|GetLocal%20Key%20Time%20Down) -1.0)))