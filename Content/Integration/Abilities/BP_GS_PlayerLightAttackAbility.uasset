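; Player light attack ability built on the Tempest state manager framework, mostly deferring to its parent class.
; When informed of a deflect, it switches the performing actor into the State.Deflected state through the state manager component and sets a flag on success.
; Start calls the parent and checks that flag without acting on it, while cancel also ends the ability.
; The query and incoming-attack functions are empty stubs returning defaults.
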(event EventInformTargetOfDeflect
  (bind _currentperformingactor (Class|TempestBaseAbilityObject|GetPerformingActor))
  (bind _returnvalue (Actor|GetComponentbyClass _currentperformingactor "/Script/TempestCombatFramework.TempestBaseStateManagerComponent"))
  (bind _returnvalue_2 (Class|TempestBaseStateManagerComponent|TryPerformStateOfClass _returnvalue (Utilities|GetClass (Class|TempestBaseStateManagerComponent|GetStateOfGameplayTag _returnvalue "(TagName=\"State.Deflected\")")) true))
  (if _returnvalue_2
    (Variables|Default|SetNewVar true)))

(event EventStartAbility
  (|CallParentFunction)
  (if (Variables|Default|GetNewVar)
    _))

(event EventCancelAbility
  (|CallParentFunction)
  (Class|TempestBaseAbilityObject|EndAbility))

(fn GetAbilityProjectile
  (return 0))

(fn GetAssociatedPassiveAbilities
  (return 0))

(fn GetBlockTimeSinceLastClicked
  (return 0.0))

(fn GetMontageCounterforAbility
  (return 0))

(fn GetMontageOfGameplayTag
  (params (Montage%20Tag :type Gameplay%20Tag%20Structure))
  (return 0))

(fn GetStrafingValues
  (return 0.0 "0, 0, 0"))

(fn ProcessIncomingAttack
  (params (Incoming%20Attack%20Type :type Gameplay%20Tag%20Structure))
  (return false))