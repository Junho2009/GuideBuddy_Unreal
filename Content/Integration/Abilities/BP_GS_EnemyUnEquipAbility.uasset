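; Enemy weapon-unequip ability (going by its name) for the Tempest combat framework, usable once the performer has no living combat target.
; It can run when the combat target is invalid, has no valid active state, or is in the Death state.
; On start it plays a random montage from the first tagged list, then applies Add modifications for the InCombat and FullyAware statuses on the performer's combat component.
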(event EventStartAbility
  (bind _currentperformingactor (Class|TempestBaseAbilityObject|GetPerformingActor))
  (bind _returnvalue (Actor|GetComponentbyClass _currentperformingactor "/TempestCombatFramework/Components/BP_TempestBaseCombatComponent.BP_TempestBaseCombatComponent_C"))
  (|CallParentFunction)
  (bind _list_of_montages (CallFunction|GetAbilityMontagesOfTag "(TagName=\"List.One\")"))
  (CallFunction|PlayAbilityMontage (.OutItem (Utilities|Array|Random _list_of_montages)) 1.0 "Duration" 0.0 "None" true)
  (Class|TempestCombatComponent|ModifyCombatStatus _returnvalue "(GameplayTags=((TagName=\"Status.Combat.InCombat\")))" "Add")
  (Class|TempestCombatComponent|ModifyCombatStatus _returnvalue "(GameplayTags=((TagName=\"Status.Combat.Fully Aware\")))" "Add"))

(fn CanPerformAbility
  (bind _currentperformingactor (Class|TempestBaseAbilityObject|GetPerformingActor))
  (bind _returnvalue (Actor|GetComponentbyClass _currentperformingactor "/Script/TempestCombatFramework.TempestCombatComponent"))
  (bind _foundcombattarget (Class|TempestCombatComponent|GetCombatTarget _returnvalue))
  (bind _returnvalue_2 (Actor|GetComponentbyClass _foundcombattarget "/Script/TempestCombatFramework.TempestBaseStateManagerComponent"))
  (bind _returnvalue_3 (Class|TempestBaseStateManagerComponent|GetCurrentActiveState _returnvalue_2))
  (Utilities|IsValid _foundcombattarget
    (:Is%20Valid
      (Utilities|IsValid _returnvalue_3
        (:Is%20Valid
          (return (== (Variables|/Script/TempestCombatFramework.TempestBaseStateObject|GetStateGameplayTag _returnvalue_3) "(TagName=\"State.Death\")")))
        (:Is%20Not%20Valid
          _)))
    (:Is%20Not%20Valid
      _))
  (return true))