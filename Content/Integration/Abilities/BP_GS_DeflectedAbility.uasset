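; BP_GS_DeflectedAbility is a gameplay ability, by its name the state a character enters when an attack is deflected.
; Its only logic is on cancel, where it calls the parent and then ends the ability.
; The projectile, passive ability, block timing, montage, strafing and incoming attack functions are empty stubs returning defaults, so the deflect behavior itself is not defined in these graphs.
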(event EventCancelAbility
  (|CallParentFunction)
  (Class|TempestBaseAbilityObject|EndAbility))

(fn GetAbilityProjectile
  (return 0))

(fn GetAssociatedPassiveAbilities
  (return 0))

(fn GetBlockTimeSinceLastClicked
  (return 0.0))

(fn GetMontageCounterforAbility
  (return 0))

(fn GetMontageOfGameplayTag
  (params (Montage%20Tag :type Gameplay%20Tag%20Structure))
  (return 0))

(fn GetStrafingValues
  (return 0.0 "0, 0, 0"))

(fn ProcessIncomingAttack
  (params (Incoming%20Attack%20Type :type Gameplay%20Tag%20Structure))
  (return false))