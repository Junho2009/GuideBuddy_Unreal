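; Character ability for being executed: plays an execution victim montage and puts the owning character into the Death state.
; It can run only while the owner is Parried and the performing actor has the Execution special property and InCombat status.
; The montage is supplied through SetTargetMontage; on start, the ability also adds InCombat to the performing actor's combat status.
; The remaining ability functions are empty stubs.
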(event EventStartAbility
  (bind _owner_character (Variables|Default|GetOwner%20Character))
  (bind _returnvalue (Actor|GetComponentbyClass _owner_character "/Script/TempestCombatFramework.TempestBaseStateManagerComponent"))
  (|CallParentFunction)
  (CallFunction|PlayAbilityMontage (Variables|Default|GetExecuted%20Montage) 1.0 "MontageLength" 0.0 "None" true)
  (Class|TempestCombatComponent|ModifyCombatStatus (Actor|GetComponentbyClass (Class|TempestBaseAbilityObject|GetPerformingActor) "/TempestCombatFramework/Components/BP_TempestBaseCombatComponent.BP_TempestBaseCombatComponent_C") "(GameplayTags=((TagName=\"Status.Combat.InCombat\")))" "Add")
  (Class|TempestBaseStateManagerComponent|SetCurrentActiveState _returnvalue (Class|TempestBaseStateManagerComponent|GetStateOfGameplayTag _returnvalue "(TagName=\"State.Death\")")))

(event EventSetTargetMontage
  (params (Anim%20Montage :type Anim%20Montage%20Object%20Reference))
  (Variables|Default|SetExecuted%20Montage Anim%20Montage))

(fn CanPerformAbility
  (bind _currentperformingactor (Class|TempestBaseAbilityObject|GetPerformingActor))
  (bind _returnvalue (Actor|GetComponentbyClass _currentperformingactor "/TempestCombatFramework/Components/BP_TempestPropertiesComponent.BP_TempestPropertiesComponent_C"))
  (if (== (Variables|/Script/TempestCombatFramework.TempestBaseStateObject|GetStateGameplayTag (Class|TempestBaseStateManagerComponent|GetCurrentActiveState (Actor|GetComponentbyClass (Variables|Default|GetOwner%20Character) "/Script/TempestCombatFramework.TempestBaseStateManagerComponent"))) "(TagName=\"State.Parried\")")
    (Utilities|IsValid _returnvalue
      (:Is%20Valid
        (bind _returnvalue_2 (Class|TempestGeneralLibrary|GetSpecialPropertyOfTag (Class|TempestPropertiesComponent|GetSpecialProperties _returnvalue) "(TagName=\"Property.Special.Behavior.Execution\")"))
        (Utilities|IsValid _returnvalue_2
          (:Is%20Valid
            (return (GameplayTags|HasTag (Class|TempestCombatComponent|GetCombatStatus (Actor|GetComponentbyClass (Class|TempestBaseAbilityObject|GetPerformingActor) "/TempestCombatFramework/Components/BP_TempestBaseCombatComponent.BP_TempestBaseCombatComponent_C")) "(TagName=\"Status.Combat.InCombat\")")))
          (:Is%20Not%20Valid
            (return false))))
      (:Is%20Not%20Valid
        (return false)))
    (else
      (return false))))

(fn GetAbilityProjectile
  (return 0))

(fn GetAssociatedPassiveAbilities
  (return 0))

(fn GetBlockTimeSinceLastClicked
  (return 0.0))

(fn GetMontageCounterforAbility
  (return 0))

(fn GetMontageOfGameplayTag
  (params (Montage%20Tag :type Gameplay%20Tag%20Structure))
  (return 0))

(fn GetStrafingValues
  (return 0.0 "0, 0, 0"))

(fn ProcessIncomingAttack
  (params (Incoming%20Attack%20Type :type Gameplay%20Tag%20Structure))
  (return false))