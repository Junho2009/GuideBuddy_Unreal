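; Katana enemy Blueprint that manages the enemy's health and lock-on widgets on top of its parent's logic.
; Active-state changes from the Tempest state manager add a health widget on equip or hit if no tagged one exists, and remove all widget components on death, execution or assassination.
; Focus toggles on TempestTargetScene create or destroy a screen-space lock-on point attached to that target.
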(event OnFocusToggled(TempestTargetScene)
  (params (bCurrentlyFocused :type Boolean))
  (if bCurrentlyFocused
    (Utilities|IsValid (Variables|Default|GetCreated%20Widget%20Component)
      (:Is%20Not%20Valid
        (bind _returnvalue (AddComponent|AddWidgetComponent false))
        (bind _output_get (Variables|Default|SetCreated%20Widget%20Component _returnvalue))
        (Class|WidgetComponent|SetWidgetSpace _output_get "Screen")
        (Class|WidgetComponent|SetDrawSize (Variables|Default|GetCreated%20Widget%20Component) "(X=30.000000,Y=30.000000)")
        (bind _returnvalue_2 (UserInterface|CreateWidget "/TempestCombatFramework/Widgets/WB_LockOnPoint.WB_LockOnPoint_C"))
        (UserInterface|SetWidget (Variables|Default|GetCreated%20Widget%20Component) _returnvalue_2)
        (Transformation|AttachComponentToComponent (Variables|Default|GetCreated%20Widget%20Component) (Variables|Default|GetTempestTargetScene) "None" "SnapToTarget" "SnapToTarget" "SnapToTarget" true)))
    (else
      (Utilities|IsValid (Variables|Default|GetCreated%20Widget%20Component)
        (:Is%20Valid
          (Components|DestroyComponent (Variables|Default|GetCreated%20Widget%20Component)))))))

(event EventOnUpdatedActiveState
  (bind _returnvalue (Actor|GetComponentbyClass "/Script/TempestCombatFramework.TempestBaseStateManagerComponent"))
  (bind _returnvalue_2 (Class|TempestBaseStateManagerComponent|GetCurrentActiveState _returnvalue))
  ;[1 0.5221 0] Widget Handling
  (|CallParentFunction)
  (Utilities|IsValid _returnvalue_2
    (:Is%20Valid
      (|SwitchGameplayTag (Variables|/Script/TempestCombatFramework.TempestBaseStateObject|GetStateGameplayTag _returnvalue_2)
        (:State.Death
          (bind _arrayelement (Utilities|Array|ReverseforEachLoop (Actor|GetComponentsByClass "/Script/UMG.WidgetComponent") :!label _label)
            (:LoopBody
              (Widget|RemovefromParent (UserInterface|GetWidget _arrayelement))
              (Components|DestroyComponent _arrayelement))))
        (:State.Executed
          (goto _label))
        (:State.Assasinated
          (goto _label))
        (:State.Equip
          (if (Utilities|Array|IsEmpty (Actor|GetComponentsbyTag "/Script/UMG.WidgetComponent" "Top Of Head Widget")) :!label _label_2
            (bind _returnvalue_3 (AddComponent|AddWidgetComponent false))
            (bind _aswb_gs_ai_health (Utilities|Casting|CastToWB_GS_AI_Health (UserInterface|GetWidget _returnvalue_3)))
            (Variables|/Game/Integration/Widgets/WB_GS_AI_Health.WB_GS_AI_Health_C|SetOwnerChracter _aswb_gs_ai_health self)
            (Default|Re-UpdateWidget _aswb_gs_ai_health)))
        (:State.Hit
          (goto _label_2))))))

(fn ConstructionScript
  (|CallParentFunction))